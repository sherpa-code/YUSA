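; Base interactable actor for the JRPG project, meant as the parent for objects, NPCs and enemies.
; InteractBegin casts itself to those child types and dispatches, but only the object path acts, calling DoInteract on a debug crystal switch.
; RotatetoFaceTarget interpolates yaw toward a location or actor, re-calling itself after a delay.
; NPC and enemy interaction, camera focus, movement stop and dialog functions are stubs or unfinished.
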(event Custom|Rotate%20to%20Face%20Target
  (params (Rotate%20to%20Face%20Type :type E_RotateToFace_Types%20Enum :default "NewEnumerator0") (Target%20World%20Location :type Vector) (Target%20Actor :type Actor%20Object%20Reference))
  (bind _returnvalue (Transformation|GetActorLocation))
  (bind _returnvalue_2 (Transformation|GetActorRotation))
  (bind _returnvalue_3 (Transformation|GetActorLocation))
  (bind _returnvalue_4 (Transformation|GetActorLocation))
  (bind _returnvalue_5 (Transformation|GetActorRotation))
  (bind _yaw (Math|Rotator|BreakRotator _returnvalue_5))
  (bind _returnvalue_6 (Math|Rotator|FindLookatRotation _returnvalue_4 Target%20World%20Location))
  (bind _returnvalue_7 (Math|Rotator|FindLookatRotation _returnvalue _returnvalue_3))
  (bind _yaw_2 (Math|Rotator|BreakRotator _returnvalue_2))
  (bind _yaw_3 (Math|Rotator|BreakRotator _returnvalue_6))
  (bind _yaw_4 (Math|Rotator|BreakRotator _returnvalue_7))
  (bind _returnvalue_8 (- _yaw_3 _yaw))
  (bind _returnvalue_9 (- _yaw_4 _yaw_2))
  (Variables|Default|SetRotateToFaceComplete? false)
  (switch Utilities|FlowControl|Switch|SwitchonE_RotateToFace_Types Rotate%20to%20Face%20Type
    (:NewEnumerator0
      (if (or (> _returnvalue_8 4.0) (< _returnvalue_8 -4.0))
        (Transformation|SetActorRotation (Math|Interpolation|RInterpTo (Transformation|GetActorRotation) (Math|Rotator|MakeRotator 0.0 0.0 _yaw_3) (Utilities|Time|GetWorldDeltaSeconds) 3.0))
        (Utilities|FlowControl|Delay 3.0 :!label _label)
        (CallFunction|RotatetoFaceTarget Rotate%20to%20Face%20Type Target%20World%20Location Target%20Actor)))
    (:NewEnumerator1
      (if (or (> _returnvalue_9 4.0) (< _returnvalue_9 -4.0))
        (Transformation|SetActorRotation (Math|Interpolation|RInterpTo (Transformation|GetActorRotation) (Math|Rotator|MakeRotator 0.0 0.0 _yaw_4) (Utilities|Time|GetWorldDeltaSeconds) 3.0))
        (goto _label)))))

(event EventBeginPlay)

(event Collision|EventActorBeginOverlap
  (params (OtherActor :type Actor%20Object%20Reference)))

(event EventTick
  (params (DeltaSeconds :type Float%20%28single-precision%29)))

(fn ConstructionScript)

(fn InteractBegin
  ;[1 1 1] Check if Interactable is Object, NPC, or Enemy
  (bind _asbp_interactable_object (Utilities|Casting|CastToBP_Interactable_Object self)
    (:then
      (CallFunction|Interact-Object _asbp_interactable_object))
    (:CastFailed
      (bind _asbp_interactable_npc (Utilities|Casting|CastToBP_Interactable_NPC self)
        (:then
          (CallFunction|Interact-NPC _asbp_interactable_npc))
        (:CastFailed
          (bind _asbp_interactable_enemy (Utilities|Casting|CastToBP_Interactable_Enemy self))
          (CallFunction|Interact-Enemy _asbp_interactable_enemy))))))

(fn Interact-Object
  (params (Target%20Interactable%20Object :type BP%20Interactable%20Object%20Object%20Reference))
  (bind _asdebug_crystal_switch_interact (Utilities|Casting|CastTodebug_CrystalSwitch_Interact Target%20Interactable%20Object))
  (Default|DoInteract _asdebug_crystal_switch_interact))

(fn Interact-Enemy
  (params (Target%20Interactable%20Enemy :type BP%20Interactable%20Enemy%20Object%20Reference)))

(fn Interact-NPC
  (params (Target%20Interactable%20NPC :type BP%20Interactable%20NPC%20Object%20Reference)))

(fn CameraFocusActor
  (params (Target%20Actor :type Actor%20Object%20Reference))
  (Variables|Default|SetisCameraInterpFinished? false))

(fn StopMovement)

(fn DialogCam-1SetAngle)

(fn DialogCall
  (params (Dialog%20Type :type E_Dialogue_Types%20Enum :default "NewEnumerator3") (Dialog%20ID%20To%20Call :type String))
  (Variables|Default|SetDialog%20ID%20To%20Call Dialog%20ID%20To%20Call)
  (Variables|Default|SetisDialogComplete? false)
  (switch Utilities|FlowControl|Switch|SwitchonE_Dialogue_Types Dialog%20Type))
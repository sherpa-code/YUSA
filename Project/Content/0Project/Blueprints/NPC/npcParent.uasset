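; Parent Blueprint for NPCs, providing shared wandering and routing interaction and dialogue calls to specific children.
; An enum switch casts self to the child: Zein Relwof for all calls, Glax Bee for interact only.
; Wandering picks a random different target point, rotates by interpolation, uses AIMoveTo, pauses, then repeats unless the player is interacting.
; Damage and death events are empty stubs with disconnected enemy logic, alongside coin-drop and health-bar functions.
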(event Custom|damageCalcApply
  (params (weaponRef :type Actor%20Object%20Reference) (actorHit :type Actor%20Object%20Reference) (damageTaken :type Integer) (damageType :type String) (lastHitChained :type Integer) (stunAmount :type Integer))
  ;[1 1 1] damageCalcApply (to self)
)

(event Custom|Death
  (params (enemyMesh :type Skeletal%20Mesh%20Component%20Object%20Reference))
  ;[1 1 1] Death
  ;;[1 1 1] Death
)

(event Custom|destroyPointLight
  (params (Owner :type Actor%20Object%20Reference) (toDestroy :type Point%20Light%20Component%20Object%20Reference) (delay :type Float%20%28single-precision%29))
  ;[1 1 1] destroyPointLight
)

(event Custom|deathAnimEnd
  ;[1 1 1] Death
  ;;[1 1 1] deathAnimEnd
)

(event Custom|NPCParent_Interact_Switch
  (params (NPC :type ENPC%20Enum :default "NewEnumerator0"))
  ;[1 1 1] NPCParent Interact Switch
  (switch Utilities|FlowControl|Switch|SwitchonENPC NPC
    (:NewEnumerator0
      (bind _asnpc_a0_bp (Utilities|Casting|CastToNPC_A0_BP self))
      (Default|NPCInteract _asnpc_a0_bp))
    (:NewEnumerator3
      (bind _asnpc_a4_bp (Utilities|Casting|CastToNPC_A4_BP self))
      (Default|NPCInteract _asnpc_a4_bp))))

(event Custom|dialogueHandler_Redirect
  (params (Method :type E_dialogueHandlerMethod%20Enum :default "NewEnumerator0"))
  ;[1 1 1] dialogueHandler_Redirect
  (switch Utilities|FlowControl|Switch|SwitchonENPC (Variables|Default|GetENPC)
    (:NewEnumerator0
      (bind _asnpc_a0_bp (Utilities|Casting|CastToNPC_A0_BP self))
      (Default|DialogueHandler _asnpc_a0_bp Method))))

(event Custom|setCrosshairVisbility
  (params (Input :type Boolean))
  ;[1 1 1] setCrosshairVisibility
)

(event Custom|dialogueContinue_Redirect
  (params (Method :type E_dialogueHandlerMethod%20Enum :default "NewEnumerator0"))
  ;[1 1 1] dialogueContinue_Redirect
  (switch Utilities|FlowControl|Switch|SwitchonENPC (Variables|Default|GetENPC)
    (:NewEnumerator0
      (bind _asnpc_a0_bp (Utilities|Casting|CastToNPC_A0_BP self))
      (Default|DialogueContinue _asnpc_a0_bp Method))))

(event EventBeginPlay
  ;[0.4948 1 0.4405] Save Reference Manager ref
  ; - Place first so refs are available
  (bind _outactors (Actor|GetAllActorswithTag "Reference Manager"))
  (bind _asreference_manager (Utilities|Casting|CastToReference_Manager (Utilities|Array|Get(acopy) _outactors)))
  (Variables|Default|SetReference%20Manager _asreference_manager))

(event Custom|ResumeTodaysSchedule
  ;[1 1 1] ResumeTodaysSchedule
  (Variables|/Game/0Project/Blueprints/NPC/A0/0rigged_animBP.0rigged_animBP_C|SetactingStateCurrent_anim (Variables|Default|GetanimBPRef) 1)
  (Variables|Default|SetisInteractingWithPC false)
  (CallFunction|TodaysSchedule))

(event Custom|RotateToFace
  (params (0Loc%20/%201Actor :type Boolean) (TargetWorldLoc :type Vector) (TargetActor :type Actor%20Object%20Reference))
  (bind _returnvalue (Transformation|GetActorLocation))
  (bind _returnvalue_2 (Transformation|GetActorRotation))
  (bind _returnvalue_3 (Transformation|GetActorLocation TargetActor))
  (bind _returnvalue_4 (Transformation|GetActorLocation))
  (bind _returnvalue_5 (Transformation|GetActorRotation))
  (bind _yaw (Math|Rotator|BreakRotator _returnvalue_5))
  (bind _returnvalue_6 (Math|Rotator|FindLookatRotation _returnvalue_4 TargetWorldLoc))
  (bind _returnvalue_7 (Math|Rotator|FindLookatRotation _returnvalue _returnvalue_3))
  (bind _yaw_2 (Math|Rotator|BreakRotator _returnvalue_2))
  (bind _yaw_3 (Math|Rotator|BreakRotator _returnvalue_6))
  (bind _yaw_4 (Math|Rotator|BreakRotator _returnvalue_7))
  (bind _returnvalue_8 (- _yaw_3 _yaw))
  (bind _returnvalue_9 (- _yaw_4 _yaw_2))
  ;[1 1 1] RotateToFace
  (if 0Loc%20/%201Actor
    (Variables|Default|SetrotateSucceed false)
    (if (or (> _returnvalue_9 4.0) (< _returnvalue_9 -4.0)) :!label _label
      (Transformation|SetActorRotation (Math|Interpolation|RInterpTo (Transformation|GetActorRotation) (Math|Rotator|MakeRotator 0.0 0.0 _yaw_4) (Utilities|Time|GetWorldDeltaSeconds) 3.0))
      (Utilities|FlowControl|Delay 0.01)
      (goto _label)
      (else
        (Variables|Default|SetrotateSucceed true)))
    (else
      (Variables|Default|SetrotateSucceed false)
      (if (or (> _returnvalue_8 4.0) (< _returnvalue_8 -4.0)) :!label _label_2
        (Transformation|SetActorRotation (Math|Interpolation|RInterpTo (Transformation|GetActorRotation) (Math|Rotator|MakeRotator 0.0 0.0 _yaw_3) (Utilities|Time|GetWorldDeltaSeconds) 3.0))
        (Utilities|FlowControl|Delay 0.01)
        (goto _label_2)
        (else
          (Variables|Default|SetrotateSucceed true))))))

(event Custom|RotThenMoveToCurrentDestLoc
  (bind _animbpref (Variables|Default|GetanimBPRef))
  ;[1 1 1] RotThenMoveToCurrentDestLoc
  (if (> (Variables|/Game/0Project/Blueprints/NPC/A0/0rigged_animBP.0rigged_animBP_C|GetSpeed (Variables|Default|GetanimBPRef)) 4.0)
    ;[1 1 1] debug
    (Development|PrintString "MoveToCurrentDest failed: already moving")
    (elif (> (Math|Vector|VectorLength (- (Variables|Default|GetcurrentDestLoc) (Transformation|GetActorLocation))) 5.0)
      (Pawn|Components|CharacterMovement|SetMovementMode (Variables|Character|GetCharacterMovement) "MOVE_Walking" 0)
      (CallFunction|RotatetoFace false (Variables|Default|GetcurrentDestLoc))
      (if (Variables|Default|GetrotateSucceed) :!label _label
        (AI|AIMoveTo (Variables|Character|GetCharacterMovement) self (Variables|Default|GetcurrentDestLoc) 0 5.0 false
          (:OnSuccess
            (Development|PrintString "Move Succeed"))
          (:OnFail
            (Development|PrintString "Move Fail")))
        (Variables|/Game/0Project/Blueprints/NPC/A0/0rigged_animBP.0rigged_animBP_C|SetactingStateCurrent_anim _animbpref 1)
        (Utilities|FlowControl|Delay (Math|Random|RandomFloatinRange 0.25 1.0))
        (if (== (Variables|/Game/0Project/Blueprints/NPC/A0/0rigged_animBP.0rigged_animBP_C|GetactingStateCurrent_anim _animbpref) 1)
          (Development|PrintString "WalkLoopEnd")
          (CallFunction|ResumeTodaysSchedule))
        (else
          (Utilities|FlowControl|Delay 0.3)
          (goto _label)))
      (else
        ;[1 1 1] debug
        (Development|PrintString "MoveToCurrentDest failed: within range of dest")))))

(event Custom|MakeTodaysSchedule
  ;[1 1 1] MakeTodaysSchedule
)

(event Custom|WanderTest-TargetPoints
  (bind _targetpointsinlevel (Variables|Default|GetTargetPointsInLevel))
  (bind _targetpointsinlevel_2 (Variables|Default|GetTargetPointsInLevel))
  ;[1 1 1] WanderTest
  ;[1 1 1] debug
  (Development|PrintString "wandertest")
  (Utilities|IsValid (Variables|Default|GetprevDestActor)
    (:Is%20Valid
      ;[1 1 1] Pick Random Dest Target That Isnt Previous One
      (bind _output_get (Variables|Default|SetcurrentDestActor (Utilities|Array|Get(acopy) _targetpointsinlevel_2 (Math|Random|RandomIntegerinRange 0 (- (Utilities|Array|Length _targetpointsinlevel_2) 1))) :!label _label))
      (if (== _output_get (Variables|Default|GetprevDestActor))
        (goto _label)
        (else
          _)))
    (:Is%20Not%20Valid
      (Variables|Default|SetcurrentDestActor (Utilities|Array|Get(acopy) _targetpointsinlevel (Math|Random|RandomIntegerinRange 0 (- (Utilities|Array|Length _targetpointsinlevel) 1))))))
  ;[1 1 1] debug
  (Development|PrintString (Utilities|GetDisplayName (Variables|Default|GetcurrentDestActor)))
  (CallFunction|RotThenMovetoCurrentDestActor))

(event Custom|RotThenMoveToCurrentDestActor
  ;[1 1 1] RotThenMoveToCurrentDestActor
  (if (> (Variables|/Game/0Project/Blueprints/NPC/A0/0rigged_animBP.0rigged_animBP_C|GetSpeed (Variables|Default|GetanimBPRef)) 4.0)
    ;[1 1 1] debug
    (Development|PrintString "MoveToCurrentDest failed: already moving")
    (else
      (Utilities|IsValid (Variables|Default|GetcurrentDestActor)
        (:Is%20Valid
          (if (> (Math|Vector|VectorLength (- (Transformation|GetActorLocation (Variables|Default|GetcurrentDestActor)) (Transformation|GetActorLocation))) 5.0)
            (if (not (Variables|Default|GetisInteractingWithPC))
              (Pawn|Components|CharacterMovement|SetMovementMode (Variables|Character|GetCharacterMovement) "MOVE_Walking" 0)
              (CallFunction|RotatetoFace true "0, 0, 0" (Variables|Default|GetcurrentDestActor))
              (if (Variables|Default|GetrotateSucceed) :!label _label
                (if (not (Variables|Default|GetisInteractingWithPC))
                  (Variables|/Game/0Project/Blueprints/NPC/A0/0rigged_animBP.0rigged_animBP_C|SetactingStateCurrent_anim (Variables|Default|GetanimBPRef) 2)
                  (AI|AIMoveTo self "0, 0, 0" (Variables|Default|GetcurrentDestActor) 5.0 false
                    (:OnSuccess
                      (Development|PrintString "Move Succeed"))
                    (:OnFail
                      (Development|PrintString "Move Fail")))
                  (if (not (Variables|Default|GetisInteractingWithPC))
                    ;[1 1 1] Idle Pause On Move Pass/Fail
                    (Variables|/Game/0Project/Blueprints/NPC/A0/0rigged_animBP.0rigged_animBP_C|SetactingStateCurrent_anim (Variables|Default|GetanimBPRef) 1)
                    (Utilities|FlowControl|Delay (Math|Random|RandomFloatinRange 0.25 1.0))
                    ;[1 1 1] Check if Idle pause was uninterrupted
                    (if (== (Variables|/Game/0Project/Blueprints/NPC/A0/0rigged_animBP.0rigged_animBP_C|GetactingStateCurrent_anim (Variables|Default|GetanimBPRef)) 1)
                      (Development|PrintString "WalkLoopEnd")
                      (if (not (Variables|Default|GetisInteractingWithPC))
                        (CallFunction|WanderTest-TargetPoints)))))
                (elif (not (Variables|Default|GetisInteractingWithPC))
                  (Utilities|FlowControl|Delay 0.3)
                  (goto _label))))
            (else
              ;[1 1 1] debug
              (Development|PrintString "MoveToCurrentDest failed: within range of dest"))))))))

(event Custom|TodaysSchedule
  ;[1 1 1] TodaysSchedule
  (Development|PrintString "Zein: TodaysSchedule")
  (if (not (Variables|Default|GetisInteractingWithPC))
    (CallFunction|WanderTest-TargetPoints)))

(fn ConstructionScript)

(fn DropCoins
  (bind _capsulecomponent (Variables|Default|GetCapsuleComponent))
  (bind _returnvalue (Transformation|GetWorldLocation _capsulecomponent))
  (if (>= (/ (Variables|Default|GetcoinsHolding) 500) 1)
    (for _index (range 1 (/ (Variables|Default|GetcoinsHolding) 500))
      (Game|SpawnActorfromClass "/Game/0Project/Blueprints/Items/coins/coin_500_bp2.coin_500_bp2_C" (Math|Transform|MakeTransform _returnvalue "0, 0, 0" "0.025000,0.025000,0.025000") "Undefined" 0 0))
    (Variables|Default|SetcoinsHolding (- (Variables|Default|GetcoinsHolding) (* 500 (/ (Variables|Default|GetcoinsHolding) 500)))))
  (if (> (/ (Variables|Default|GetcoinsHolding) 100) 0)
    (for _index_2 (range 1 (/ (Variables|Default|GetcoinsHolding) 100))
      (Game|SpawnActorfromClass "/Game/0Project/Blueprints/Items/coins/coin_100_bp2.coin_100_bp2_C" (Math|Transform|MakeTransform _returnvalue "0, 0, 0" "0.017500,0.017500,0.017500") "Undefined" 0 0))
    (Variables|Default|SetcoinsHolding (- (Variables|Default|GetcoinsHolding) (* 100 (/ (Variables|Default|GetcoinsHolding) 100)))))
  (if (> (/ (Variables|Default|GetcoinsHolding) 50) 0)
    (for _index_3 (range 1 (/ (Variables|Default|GetcoinsHolding) 50))
      (Game|SpawnActorfromClass "/Game/0Project/Blueprints/Items/coins/coin_50_BP2.coin_50_BP2_C" (Math|Transform|MakeTransform _returnvalue "0, 0, 0" "0.012500,0.012500,0.012500") "Undefined" 0 0))
    (Variables|Default|SetcoinsHolding (- (Variables|Default|GetcoinsHolding) (* 50 (/ (Variables|Default|GetcoinsHolding) 50)))))
  (if (> (/ (Variables|Default|GetcoinsHolding) 10) 0)
    (for _index_4 (range 1 (/ (Variables|Default|GetcoinsHolding) 10))
      (Game|SpawnActorfromClass "/Game/0Project/Blueprints/Items/coins/coin_10_BP.coin_10_BP_C" (Math|Transform|MakeTransform _returnvalue "0, 0, 0" "0.010000,0.010000,0.010000") "Undefined" 0 0))))

(fn StatsUpdate
  (bind _hp_max (Variables|Default|GetHP_Max))
  (bind _hp_current (Variables|Default|GetHP_Current))
  (bind _returnvalue (Math|Conversions|ToFloat(Integer) _hp_current))
  (bind _returnvalue_2 (Math|Conversions|ToFloat(Integer) _hp_max))
  (bind _returnvalue_3 (/ _returnvalue _returnvalue_2))
  (bind _returnvalue_4 (Math|Float|Clamp(Float) _returnvalue_3))
  (bind _asenemy_hp_2 (Utilities|Casting|CastToEnemyHP_2 (UserInterface|GetUserWidgetObject (Variables|Default|GetEnemyHPWidget))))
  (Progress|SetPercent (Variables|/Game/0Project/Blueprints/Widgets/EnemyHP_2.EnemyHP_2_C|GetHealth_Bar _asenemy_hp_2) _returnvalue_4)
  (Variables|Default|SetHealth_Pct _returnvalue_4)
  (Progress|SetPercent (Variables|/Game/0Project/Blueprints/Widgets/EnemyHP_2.EnemyHP_2_C|GetStun_Bar _asenemy_hp_2) (Math|Float|Clamp(Float) (/ (Math|Conversions|ToFloat(Integer) 0) (Math|Conversions|ToFloat(Integer) 0)))))
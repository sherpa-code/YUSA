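; Player controller that caches the Reference Manager actor on BeginPlay, found by tag, and uses it to reach the Dialogue Manager.
; Pressing B shows a hardcoded dialogue popup announcing an absorbed Magma Anima with its finisher and skill, or prints a fallback string without a manager.
; A Delay loop polls until the popup closes, then restores walking and game-only input and removes the widget.
; Older Yusa-character dialogue nodes remain unconnected.
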(event EventBeginPlay
  ;[1 1 1] Event BeginPlay
  (Utilities|FlowControl|Sequence
    (:then_0
      ;[0.4948 1 0.4405] Save Reference Manager ref
      (bind _outactors (Actor|GetAllActorswithTag "Reference Manager"))
      (bind _asreference_manager (Utilities|Casting|CastToReference_Manager (Utilities|Array|Get(acopy) _outactors)))
      (Variables|Default|SetReference%20Manager _asreference_manager))
    (:then_1)
    (:then_2)
    (:then_3)
    (:then_4)))

(event Input|KeyboardEvents|B
  (params (Key :type Key%20Structure))
  (bind _reference_manager (Variables|Default|GetReference%20Manager))
  (bind _dialogue_manager (Variables|/Game/0Project/Blueprints/0-Managers/Reference_Manager.Reference_Manager_C|GetDialogue%20Manager _reference_manager))
  ;[1 1 1] B Key
  (:Pressed
    (Utilities|IsValid _dialogue_manager
      (:Is%20Valid
        (Default|DialoguePopup-Create _dialogue_manager)
        (Default|DialoguePopup-AddScripts (Variables|/Game/0Project/Blueprints/0-Managers/Reference_Manager.Reference_Manager_C|GetDialogue%20Manager (Variables|Default|GetReference%20Manager)) "" "" (Utilities|Array|MakeArray "    You absorbed: 
    ~Magma Anima~" "    Finisher: 
           Molten Slash 
    Skill: 
           Lava Glow"))
        (Default|DialoguePopup-ClearandPrintScripts (Variables|/Game/0Project/Blueprints/0-Managers/Reference_Manager.Reference_Manager_C|GetDialogue%20Manager (Variables|Default|GetReference%20Manager)) "NewEnumerator0")
        ;[1 1 1] Wait for dialogue completion
        (if (Variables|/Game/0Project/Blueprints/0-Managers/Dialogue_Manager.Dialogue_Manager_C|GetIs%20Any%20Dialogue%20Popup%20Open? (Variables|/Game/0Project/Blueprints/0-Managers/Reference_Manager.Reference_Manager_C|GetDialogue%20Manager (Variables|Default|GetReference%20Manager))) :!label _label
          (Utilities|FlowControl|Delay 0.6)
          (goto _label)
          (else
            (Pawn|Components|CharacterMovement|SetMovementMode (Variables|/Script/Engine.Character|GetCharacterMovement (Game|GetPlayerCharacter 0)) "MOVE_Walking" 0)
            (Input|SetInputModeGameOnly (Game|GetPlayerController 0))
            (Widget|RemovefromParent (Variables|/Game/0Project/Blueprints/0-Managers/Dialogue_Manager.Dialogue_Manager_C|GetdialoguePopRef_current (Variables|/Game/0Project/Blueprints/0-Managers/Reference_Manager.Reference_Manager_C|GetDialogue%20Manager (Variables|Default|GetReference%20Manager)))))))
      (:Is%20Not%20Valid
        (Development|PrintString "Hello")))))

(fn ConstructionScript)
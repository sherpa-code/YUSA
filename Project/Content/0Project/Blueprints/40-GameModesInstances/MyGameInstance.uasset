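; MyGameInstance is a game instance Blueprint that switches game modes by opening a named map.
; GameModeSwitcherEvent compares the requested mode with the current one and, for mode 1, calls SwitchToLevelModeEvent to load the level.
; The current mode is assigned to itself, so the switch never stores the requested mode.
; Battle, town and world events are empty old-project stubs, with unconnected logic for saving player location and returning levels.
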(event Custom|SwitchToLevelModeEvent
  (params (MapSwitchTo :type Name))
  ;[1 1 1] GameMode Switcher
  (Game|OpenLevel(byName) MapSwitchTo))

(event Custom|SwitchToTownModeEvent
  ;[1 1 1] FROM OLD PROJECT
)

(event Custom|SwitchToBattleModeEvent
  (params (BattleZone :type Name))
  ;[1 1 1] FROM OLD PROJECT
)

(event Custom|SwitchToWorldModeEvent
  ;[1 1 1] FROM OLD PROJECT
)

(event Custom|GameModeSwitcherEvent
  (params (GameModeSwitchTo :type Integer) (MapSwitchTo :type Name))
  (bind _gamemodecurrent (Variables|Default|GetGameModeCurrent))
  ;[1 1 1] GameMode Switcher
  (if (!= _gamemodecurrent GameModeSwitchTo)
    (Variables|Default|SetgameModeCurrent _gamemodecurrent)
    (switch int GameModeSwitchTo
      (:1
        (CallFunction|SwitchtoLevelModeEvent MapSwitchTo)))))
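; GM_Wild is the game mode for the Wild area, providing events to show the Wild HUD and run a world clock.
; WorldClock toggles a looping timer that advances one in-game minute per second, rolling into hours and days in MyGameInstance's Time.
; Each tick passes the new time to WildHUDv2's TimeFontAssembler for display.
; BeginPlay is empty, so nothing here starts the HUD or clock.
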(event Custom|WorldClock
  (params (Enable/Disable :type Boolean))
  ;[1 0.7553 0] IMPORTED FROM GameMode_Wild
  ;;[1 1 1] World Clock
  ;;;[1 1 1] WorldClock
  (if Enable/Disable
    (if (Variables|Default|GetisWorldClockActive?)
      (Development|PrintString "WorldClock already active.")
      (else
        (Utilities|Time|SetTimerbyFunctionName 0 "WorldClock-Tick" 1.0 true)
        (Variables|Default|SetisWorldClockActive? true)))
    (elif (Variables|Default|GetisWorldClockActive?)
      (Utilities|Time|ClearTimerbyFunctionName 0 "WorldClock-Tick")
      (Variables|Default|SetisWorldClockActive? false)
      (else
        (Development|PrintString "WorldClock not active.")))))

(event Custom|CreateDisplayWildHUD
  ;[1 0.7553 0] IMPORTED FROM GameMode_Wild
  ;;[1 1 1] CreateDisplayWildHUD
  (bind _returnvalue (UserInterface|CreateWidget "/Game/0Project/Blueprints/HUDs/WildHUDv2.WildHUDv2_C" (Game|GetPlayerController 0)))
  (UserInterface|Viewport|AddtoViewport (stale _returnvalue) 0)
  (Variables|Default|SetWildHUD2_ref _returnvalue))

(event Custom|WorldClock-Tick
  ;[1 0.7553 0] IMPORTED FROM GameMode_Wild
  ;;[1 1 1] World Clock
  ;;;[1 1 1] WorldClock-Tick
  (bind _asmy_game_instance (Utilities|Casting|CastToMyGameInstance (Game|GetGameInstance)))
  (bind _result (Math|Integer|IncrementInt (.Minutes (Utilities|Struct|BreakFTime (Variables|/Game/0Project/Blueprints/40-GameModesInstances/MyGameInstance.MyGameInstance_C|GetTime _asmy_game_instance))))
    (:%20%20
      (if (== _result 60)
        (bind _result_2 (Math|Integer|IncrementInt (.Hours (Utilities|Struct|BreakFTime (Variables|/Game/0Project/Blueprints/40-GameModesInstances/MyGameInstance.MyGameInstance_C|GetTime _asmy_game_instance))))
          (:%20%20
            (if (== _result_2 24)
              (bind _result_3 (Math|Integer|IncrementInt (.Days (Utilities|Struct|BreakFTime (Variables|/Game/0Project/Blueprints/40-GameModesInstances/MyGameInstance.MyGameInstance_C|GetTime _asmy_game_instance))))
                (:%20%20
                  (bind _output_get (Variables|/Game/0Project/Blueprints/40-GameModesInstances/MyGameInstance.MyGameInstance_C|SetTime _asmy_game_instance (Utilities|Struct|MakeFTime _result_3 0)))
                  (Default|TimeFontAssembler (Variables|Default|GetWildHUD2_ref) _output_get)))
              (else
                (bind _output_get_2 (Variables|/Game/0Project/Blueprints/40-GameModesInstances/MyGameInstance.MyGameInstance_C|SetTime _asmy_game_instance (Utilities|Struct|MakeFTime (.Days (Utilities|Struct|BreakFTime (Variables|/Game/0Project/Blueprints/40-GameModesInstances/MyGameInstance.MyGameInstance_C|GetTime _asmy_game_instance))) _result_2)))
                (Default|TimeFontAssembler (Variables|Default|GetWildHUD2_ref) _output_get_2)))))
        (else
          (bind _output_get_3 (Variables|/Game/0Project/Blueprints/40-GameModesInstances/MyGameInstance.MyGameInstance_C|SetTime _asmy_game_instance (Utilities|Struct|MakeFTime (.Days (Utilities|Struct|BreakFTime (Variables|/Game/0Project/Blueprints/40-GameModesInstances/MyGameInstance.MyGameInstance_C|GetTime _asmy_game_instance))) (.Hours (Utilities|Struct|BreakFTime (Variables|/Game/0Project/Blueprints/40-GameModesInstances/MyGameInstance.MyGameInstance_C|GetTime _asmy_game_instance))) _result)))
          (Default|TimeFontAssembler (Variables|Default|GetWildHUD2_ref) _output_get_3))))))

(event EventBeginPlay
  ;[1 0.7553 0] IMPORTED FROM GameMode_Wild
  ;;[1 1 1] BeginPlay
)

(event EventTick
  (params (DeltaSeconds :type Float%20%28single-precision%29)))

(fn ConstructionScript
  (|CallParentFunction))
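; Base interactable actor that makes itself known to the player character class char1 when that character is within range.
; Begin and end overlaps on InteractableArea register and unregister the actor with char1 through its interactable message functions, with debug prints on entry.
; SetHighlight toggles Render Custom Depth on the Mesh for highlighting; nothing in this graph calls it.
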(event OnComponentBeginOverlap(InteractableArea)
  (params (OverlappedComponent :type Primitive%20Component%20Object%20Reference) (OtherActor :type Actor%20Object%20Reference) (OtherComp :type Primitive%20Component%20Object%20Reference) (OtherBodyIndex :type Integer) (bFromSweep :type Boolean) (SweepResult :type Hit%20Result%20Structure%20%28by%20ref%29))
  (bind _aschar_1 (Utilities|Casting|CastTochar1 OtherActor)
    (:then
      (Development|PrintString "yes")
      (Class|BPIInteract|RegisterInteractable(Message) _aschar_1 self))
    (:CastFailed
      (Development|PrintString "no"))))

(event OnComponentEndOverlap(InteractableArea)
  (params (OverlappedComponent :type Primitive%20Component%20Object%20Reference) (OtherActor :type Actor%20Object%20Reference) (OtherComp :type Primitive%20Component%20Object%20Reference) (OtherBodyIndex :type Integer))
  (bind _aschar_1 (Utilities|Casting|CastTochar1 OtherActor))
  (Class|BPIInteract|UnregisterInteractable(Message) _aschar_1 self))

(event EventBeginPlay)

(event Collision|EventActorBeginOverlap
  (params (OtherActor :type Actor%20Object%20Reference)))

(event EventTick
  (params (DeltaSeconds :type Float%20%28single-precision%29)))

(fn ConstructionScript)

(fn SetHighlight
  (params (Hightlight? :type Boolean))
  (Rendering|SetRenderCustomDepth (Variables|Character|GetMesh) Hightlight?))
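; Manager that builds the JRPG HUD by game mode and provides popup widget helpers; only the Battle HUD is implemented, with Town, Wild and World left as stubs.
; The Battle HUD gets an IP Gauge marker per living combatant, cross-linked to it, and a stats row per party member, using data from the Reference Manager.
; Popup helpers position widgets by screen presets and toggle menu buttons, but the ref-saving logic is disconnected.
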(event EventBeginPlay
  ;[1 1 1] Event BeginPlay
  (Utilities|FlowControl|Sequence
    (:then_0
      ;[0.4948 1 0.4405] Save Reference Manager ref
      ; - Place first so refs are available
      (bind _outactors (Actor|GetAllActorswithTag "Reference Manager"))
      (bind _asjrpg_reference_manager (Utilities|Casting|CastToJRPG_Reference_Manager (Utilities|Array|Get(acopy) _outactors)))
      (Variables|Default|SetReference%20Manager _asjrpg_reference_manager))
    (:then_1)))

(fn ConstructionScript)

(fn ClearWidgetPopupRefs
  ;[1 1 1] Delete local refs to Popup widgets
  ;;[1 1 1] Debug Popup refs
  (Variables|PopupDynamic|SetWidget%20Popup%20ref 0)
  (Variables|PopupDynamic|SetWidget%20Popup%20Dynamic%20ref 0))

(fn SaveWidgetPopupRefs
  (params (Popup%20ref :type User%20Widget%20Object%20Reference)))

(fn SetScreenPositionOfWidget
  ;[1 1 1] X-position Presets
  (switch Utilities|FlowControl|Switch|SwitchonE_Popup_X_Position_Presets (Variables|PopupWidgetVariables|GetX-position%20Preset)
    (:NewEnumerator0
      (Variables|PopupWidgetVariables|SetPopup_align_calc "(X=0.000000,Y=-0.500000)"))
    (:NewEnumerator3
      (Variables|PopupWidgetVariables|SetPopup_align_calc "(X=-0.250000,Y=-0.500000)"))
    (:NewEnumerator4
      (Variables|PopupWidgetVariables|SetPopup_align_calc "(X=-0.400000,Y=-0.500000)"))
    (:NewEnumerator5
      (Variables|PopupWidgetVariables|SetPopup_align_calc "(X=-0.550000,Y=-0.500000)"))
    (:NewEnumerator9
      (Variables|PopupWidgetVariables|SetPopup_align_calc "(X=-0.700000,Y=-0.500000)"))
    (:NewEnumerator10
      (Variables|PopupWidgetVariables|SetPopup_align_calc "(X=-0.900000,Y=-0.500000)"))
    (:NewEnumerator11
      (Variables|PopupWidgetVariables|SetPopup_align_calc "(X=-1.050000,Y=-0.500000)"))
    (:NewEnumerator16
      (Variables|PopupWidgetVariables|SetPopup_align_calc "(X=-1.200000,Y=-0.500000)"))
    (:NewEnumerator15
      (Variables|PopupWidgetVariables|SetPopup_align_calc "(X=-1.350000,Y=-0.500000)"))
    (:NewEnumerator20
      (Variables|PopupWidgetVariables|SetPopup_align_calc "(X=-1.500000,Y=-0.500000)"))
    (:NewEnumerator2
      (Variables|PopupWidgetVariables|SetPopup_align_calc "(X=-1.700000,Y=-0.500000)"))
    (:NewEnumerator19
      (Variables|PopupWidgetVariables|SetPopup_align_calc "(X=-1.900000,Y=-0.500000)"))
    (:NewEnumerator18
      (Variables|PopupWidgetVariables|SetPopup_align_calc "(X=-2.050000,Y=-0.500000)"))
    (:NewEnumerator17
      (Variables|PopupWidgetVariables|SetPopup_align_calc "(X=-2.200000,Y=-0.500000)"))
    (:NewEnumerator14
      (Variables|PopupWidgetVariables|SetPopup_align_calc "(X=-2.350000,Y=-0.500000)"))
    (:NewEnumerator13
      (Variables|PopupWidgetVariables|SetPopup_align_calc "(X=-2.500000,Y=-0.500000)"))
    (:NewEnumerator12
      (Variables|PopupWidgetVariables|SetPopup_align_calc "(X=-2.650000,Y=-0.500000)"))
    (:NewEnumerator8
      (Variables|PopupWidgetVariables|SetPopup_align_calc "(X=-2.800000,Y=-0.500000)"))
    (:NewEnumerator7
      (Variables|PopupWidgetVariables|SetPopup_align_calc "(X=-2.950000,Y=-0.500000)"))
    (:NewEnumerator6
      (Variables|PopupWidgetVariables|SetPopup_align_calc "(X=-3.100000,Y=-0.500000)"))
    (:NewEnumerator1
      (Variables|PopupWidgetVariables|SetPopup_align_calc "(X=-3.250000,Y=-0.500000)")))
  ;[1 1 1] Y-position Presets
  (switch Utilities|FlowControl|Switch|SwitchonE_Popup_Y_Position_Presets (Variables|PopupWidgetVariables|GetY-position%20Preset)
    (:NewEnumerator4
      (Variables|PopupWidgetVariables|SetPopup_XY_calc (Math|Vector2D|MakeVector2D (.X (Math|Vector2D|BreakVector2D (Variables|PopupWidgetVariables|GetPopup_XY_calc))) -3.2e+02)))
    (:NewEnumerator2
      (Variables|PopupWidgetVariables|SetPopup_XY_calc (Math|Vector2D|MakeVector2D (.X (Math|Vector2D|BreakVector2D (Variables|PopupWidgetVariables|GetPopup_XY_calc))) -3e+02)))
    (:NewEnumerator1
      (Variables|PopupWidgetVariables|SetPopup_XY_calc (Math|Vector2D|MakeVector2D (.X (Math|Vector2D|BreakVector2D (Variables|PopupWidgetVariables|GetPopup_XY_calc))) -2.8e+02)))
    (:NewEnumerator0
      (Variables|PopupWidgetVariables|SetPopup_XY_calc (Math|Vector2D|MakeVector2D (.X (Math|Vector2D|BreakVector2D (Variables|PopupWidgetVariables|GetPopup_XY_calc))) -2.5e+02)))
    (:NewEnumerator3
      (Variables|PopupWidgetVariables|SetPopup_XY_calc (Math|Vector2D|MakeVector2D (.X (Math|Vector2D|BreakVector2D (Variables|PopupWidgetVariables|GetPopup_XY_calc))) 375.0))))
  (Utilities|Casting|CastToW_Popup_Dynamic (Variables|PopupDynamic|GetWidget%20Popup%20ref)
    (:then
      ;[1 1 1] Set Position and Alignment
      (Class|UserWidget|SetPositioninViewport (Variables|PopupDynamic|GetWidget%20Popup%20ref) (Variables|PopupWidgetVariables|GetPopup_XY_calc) true)
      (Class|UserWidget|SetAlignmentinViewport (Variables|PopupDynamic|GetWidget%20Popup%20ref) (Variables|PopupWidgetVariables|GetPopup_align_calc)))
    (:CastFailed
      (Utilities|Casting|CastToW_Popup_YesNo (Variables|PopupDynamic|GetWidget%20Popup%20ref))
      ;[1 1 1] Set Position and Alignment
      (Class|UserWidget|SetPositioninViewport (Variables|PopupDynamic|GetWidget%20Popup%20Debug%20YesNo%20ref) (Variables|PopupWidgetVariables|GetPopup_XY_calc) true)
      (Class|UserWidget|SetAlignmentinViewport (Variables|PopupDynamic|GetWidget%20Popup%20Debug%20YesNo%20ref) (Variables|PopupWidgetVariables|GetPopup_align_calc)))))

(fn Enable/DisableMenuButtons
  (params (Enable%20/%20Disable :type E_Enable_Disable%20Enum :default "NewEnumerator0") (Target%20Widget :type User%20Widget%20Object%20Reference))
  ;[1 1 1] Enable / Disable Buttons
  (Variables|PopupDynamic|SetWidget%20Popup%20ref%20-%20Enable/Disable%20Target Target%20Widget)
  (switch Utilities|FlowControl|Switch|SwitchonE_Enable_Disable Enable%20/%20Disable
    (:NewEnumerator0
      ;[1 1 1] Enable all Menu Items
      (for _array_element (Variables|/Game/3-JRPGProjectImport/0-Blueprints/30-Widgets/W_Popup_Dynamic.W_Popup_Dynamic_C|GetMenu%20Items (Variables|PopupDynamic|GetWidget%20Popup%20Dynamic%20ref))
        (Widget|SetIsEnabled (Variables|/Game/3-JRPGProjectImport/0-Blueprints/30-Widgets/W_MenuItem.W_MenuItem_C|GetMenuItemButtonref _array_element) true)))
    (:NewEnumerator3
      ;[1 1 1] Disable and Hide all Menu Items and their children Buttons
      (for _array_element_2 (Variables|/Game/3-JRPGProjectImport/0-Blueprints/30-Widgets/W_Popup_Dynamic.W_Popup_Dynamic_C|GetMenu%20Items (Variables|PopupDynamic|GetWidget%20Popup%20Dynamic%20ref))
        (Widget|SetIsEnabled (Variables|/Game/3-JRPGProjectImport/0-Blueprints/30-Widgets/W_MenuItem.W_MenuItem_C|GetMenuItemButtonref _array_element_2) false)
        (Widget|SetVisibility (Variables|/Game/3-JRPGProjectImport/0-Blueprints/30-Widgets/W_MenuItem.W_MenuItem_C|Gethighlighted_backing _array_element_2) "Hidden")))))

(fn MakeHUD
  (params (Target%20Game%20Mode :type E_Game_Modes%20Enum :default "NewEnumerator0"))
  (switch Utilities|FlowControl|Switch|SwitchonE_Game_Modes Target%20Game%20Mode
    (:NewEnumerator0
      (CallFunction|MakeHUD-Town))
    (:NewEnumerator3
      (CallFunction|MakeHUD-Wild))
    (:NewEnumerator1
      (CallFunction|MakeHUD-World))
    (:NewEnumerator2
      (CallFunction|MakeHUD-Battle))))

(fn MakeHUD-Battle
  ;[1 1 1] Create HUD Battle widget
  (bind _returnvalue (UserInterface|CreateWidget "/Game/3-JRPGProjectImport/0-Blueprints/30-Widgets/6-HUDs/HUD_Battle.HUD_Battle_C" (Game|GetPlayerController 0)))
  (bind _output_get (Variables|Default|SetCurrent%20HUD _returnvalue))
  ;[1 1 1] Save IP Gauge ref
  (bind _ashud_battle (Utilities|Casting|CastToHUD_Battle _output_get))
  (bind _output_get_2 (Variables|Default|SetBattle%20-%20IP%20Gauge (Variables|/Game/3-JRPGProjectImport/0-Blueprints/30-Widgets/6-HUDs/HUD_Battle.HUD_Battle_C|GetW_IP_Gauge _ashud_battle)))
  ;[1 1 1] Populate IP Gauge
  (CallFunction|MakeHUD-Battle-PopulateIPGauge)
  ;[1 1 1] Populate Stats
  (CallFunction|MakeHUD-Battle-PopulateStats)
  ;[1 1 1] Add to Viewport
  (UserInterface|Viewport|AddtoViewport (Variables|Default|GetCurrent%20HUD) 0))

(fn MakeHUD-Town)

(fn MakeHUD-Wild)

(fn MakeHUD-World)

(fn MakeHUD-Battle-PopulateStats
  ;[1 1 1] for each Party Character that is not None
  (for (_array_element _array_index) (Variables|/Game/3-JRPGProjectImport/0-Blueprints/JRPG_MyGameInstance.JRPG_MyGameInstance_C|GetParty%20Playable%20Characters (Variables|/Game/3-JRPGProjectImport/0-Blueprints/JRPG_Reference_Manager.JRPG_Reference_Manager_C|GetMyGameInstance (Variables|Default|GetReference%20Manager)))
    (if (Utilities|Enum|NotEqual(Enum) _array_element "NewEnumerator1")
      (Variables|Default|SetCurrent%20Index _array_index)
      (bind _returnvalue (UserInterface|CreateWidget "/Game/3-JRPGProjectImport/0-Blueprints/30-Widgets/4-Combat/W_Battle_HUD_Stats_Element.W_Battle_HUD_Stats_Element_C" (Variables|/Game/3-JRPGProjectImport/0-Blueprints/JRPG_Reference_Manager.JRPG_Reference_Manager_C|GetPC%20Controller (Variables|Default|GetReference%20Manager))))
      (Variables|Default|SetTarget%20HUD%20Stats _returnvalue)
      (bind _ashud_battle (Utilities|Casting|CastToHUD_Battle (Variables|Default|GetCurrent%20HUD)))
      (Widget|Panel|AddChild (Variables|/Game/3-JRPGProjectImport/0-Blueprints/30-Widgets/4-Combat/W_Battle_HUD_Stats.W_Battle_HUD_Stats_C|GetVerticalBox_Stats (Variables|/Game/3-JRPGProjectImport/0-Blueprints/30-Widgets/6-HUDs/HUD_Battle.HUD_Battle_C|GetW_Battle_HUD_Stats _ashud_battle)) (Variables|Default|GetTarget%20HUD%20Stats))
      (bind _asw_battle_hud_stats_element (Utilities|Casting|CastToW_Battle_HUD_Stats_Element (Variables|Default|GetTarget%20HUD%20Stats)))
      (CallFunction|MakeHUD-Battle-SetElementStats _asw_battle_hud_stats_element (.Name (Utilities|Struct|BreakS_Character_Stats (Utilities|Array|Get(acopy) (Variables|/Game/3-JRPGProjectImport/0-Blueprints/JRPG_MyGameInstance.JRPG_MyGameInstance_C|GetPC%20Stats (Variables|/Game/3-JRPGProjectImport/0-Blueprints/JRPG_Reference_Manager.JRPG_Reference_Manager_C|GetMyGameInstance (Variables|Default|GetReference%20Manager))) (Variables|Default|GetCurrent%20Index)))) (Utilities|String|ToString(Integer) (.HPCurrent (Utilities|Struct|BreakS_Character_Stats (Utilities|Array|Get(acopy) (Variables|/Game/3-JRPGProjectImport/0-Blueprints/JRPG_MyGameInstance.JRPG_MyGameInstance_C|GetPC%20Stats (Variables|/Game/3-JRPGProjectImport/0-Blueprints/JRPG_Reference_Manager.JRPG_Reference_Manager_C|GetMyGameInstance (Variables|Default|GetReference%20Manager))) (Variables|Default|GetCurrent%20Index))))) (Utilities|String|ToString(Integer) (.MPCurrent (Utilities|Struct|BreakS_Character_Stats (Utilities|Array|Get(acopy) (Variables|/Game/3-JRPGProjectImport/0-Blueprints/JRPG_MyGameInstance.JRPG_MyGameInstance_C|GetPC%20Stats (Variables|/Game/3-JRPGProjectImport/0-Blueprints/JRPG_Reference_Manager.JRPG_Reference_Manager_C|GetMyGameInstance (Variables|Default|GetReference%20Manager))) (Variables|Default|GetCurrent%20Index)))))))))

(fn MakeHUD-Battle-SetElementStats
  (params (Stats%20Item :type W%20Battle%20HUD%20Stats%20Element%20Object%20Reference) (Name :type String) (HP :type String) (MP :type String))
  (bind _reference_manager (Variables|Default|GetReference%20Manager))
  (bind _current_index (Variables|Default|GetCurrent%20Index))
  (bind _mygameinstance (Variables|/Game/3-JRPGProjectImport/0-Blueprints/JRPG_Reference_Manager.JRPG_Reference_Manager_C|GetMyGameInstance _reference_manager))
  (bind _pc_stats (Variables|/Game/3-JRPGProjectImport/0-Blueprints/JRPG_MyGameInstance.JRPG_MyGameInstance_C|GetPC%20Stats _mygameinstance))
  (bind _output (Utilities|Array|Get(acopy) _pc_stats _current_index))
  (bind (_name _hpcurrent _hpmax) (Utilities|Struct|BreakS_Character_Stats _output))
  (Rendering|Components|TextRender|SetText (Variables|/Game/3-JRPGProjectImport/0-Blueprints/30-Widgets/4-Combat/W_Battle_HUD_Stats_Element.W_Battle_HUD_Stats_Element_C|GetNameText Stats%20Item) (Utilities|Text|ToText(String) Name))
  (Rendering|Components|TextRender|SetText (Variables|/Game/3-JRPGProjectImport/0-Blueprints/30-Widgets/4-Combat/W_Battle_HUD_Stats_Element.W_Battle_HUD_Stats_Element_C|GetHPNum Stats%20Item) (Utilities|Text|ToText(String) HP))
  (Rendering|Components|TextRender|SetText (Variables|/Game/3-JRPGProjectImport/0-Blueprints/30-Widgets/4-Combat/W_Battle_HUD_Stats_Element.W_Battle_HUD_Stats_Element_C|GetMPNum Stats%20Item) (Utilities|Text|ToText(String) MP))
  (if (< _hpcurrent _hpmax)
    (Progress|SetPercent (Variables|/Game/3-JRPGProjectImport/0-Blueprints/30-Widgets/4-Combat/W_Battle_HUD_Stats_Element.W_Battle_HUD_Stats_Element_C|GetHPBar Stats%20Item) (/ (Math|Conversions|ToFloat(Integer) _hpcurrent) (Math|Conversions|ToFloat(Integer) _hpmax)))))

(fn MakeHUD-Battle-PopulateIPGauge
  ;[1 1 1] Battle - Populate IP Gauge
  ;[1 1 1] For each Combatant alive...
  (for _array_element (Variables|/Game/3-JRPGProjectImport/0-Blueprints/40-GameModesInstances/JRPG_GM_Battle.JRPG_GM_Battle_C|GetCombatants%20Alive (Variables|/Game/3-JRPGProjectImport/0-Blueprints/JRPG_Reference_Manager.JRPG_Reference_Manager_C|GetGame%20Mode%20Battle%20ref (Variables|Default|GetReference%20Manager)))
    ;[1 1 1] Create IP Gauge Marker
    (bind _returnvalue (UserInterface|CreateWidget "/Game/3-JRPGProjectImport/0-Blueprints/30-Widgets/5-IP_Gauge/W_IP_Gauge_Marker_Combatant.W_IP_Gauge_Marker_Combatant_C" (Game|GetPlayerController 0)))
    ;[1 1 1] On the combatant (parent character), save a ref to it's corresponding Marker
    (Variables|/Game/3-JRPGProjectImport/0-Blueprints/6-Characters/JRPG_Parent_Character.JRPG_Parent_Character_C|SetBattle%20-%20My%20IP%20Gauge%20Marker _array_element _returnvalue)
    ;[1 1 1] Set Name on Marker
    (Rendering|Components|TextRender|SetText (Variables|/Game/3-JRPGProjectImport/0-Blueprints/30-Widgets/5-IP_Gauge/W_IP_Gauge_Marker_Combatant.W_IP_Gauge_Marker_Combatant_C|GetMarkerCharacterName _returnvalue) (Utilities|Text|ToText(String) (.Name (Utilities|Struct|BreakS_Character_Stats (Variables|/Game/3-JRPGProjectImport/0-Blueprints/6-Characters/JRPG_Parent_Character.JRPG_Parent_Character_C|GetCharacter%20Stats _array_element)))))
    ;[1 1 1] Add as child to the Marker Area (canvas panel) on the IP Gauge
    (Widget|Panel|AddChild (Variables|/Game/3-JRPGProjectImport/0-Blueprints/30-Widgets/5-IP_Gauge/W_IP_Gauge.W_IP_Gauge_C|GetIPGaugeMeterArea (Variables|Default|GetBattle%20-%20IP%20Gauge)) _returnvalue)
    ;[1 1 1] On the Marker itself, save ref to the combatant it refers to
    (Variables|/Game/3-JRPGProjectImport/0-Blueprints/30-Widgets/5-IP_Gauge/W_IP_Gauge_Marker_Combatant.W_IP_Gauge_Marker_Combatant_C|SetCombatant%20ref _returnvalue _array_element)))

(fn SetHUDPositionRelativetoViewport)
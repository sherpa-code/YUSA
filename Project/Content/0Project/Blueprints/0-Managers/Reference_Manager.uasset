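; Reference manager that caches references to the game's core objects in its own variables at BeginPlay.
; SaveAllReferences runs a sequence storing the game instance, player controller and parent game mode, plus its Town or Wild subclass after clearing both.
; Camera, popup widget, HUD and dialogue managers and the player character are found by actor tag, taking the first match and casting it.
; Most missing-reference debug prints are disconnected, so those lookups fail silently.
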(event EventBeginPlay
  (CallFunction|SaveAllReferences))

(fn ConstructionScript)

(fn SaveAllReferences
  (Utilities|FlowControl|Sequence
    (:then_1
      ;[1 1 1] MyGameInstance
      (bind _asmy_game_instance (Utilities|Casting|CastToMyGameInstance (Game|GetGameInstance))
        (:then
          (Variables|Default|SetMyGameInstance _asmy_game_instance))
        (:CastFailed
          ;[1 1 1] DEBUG
          (Development|PrintString "RefMan: MyGameInstance is not valid A")
          (Utilities|IsValid (Variables|Default|GetMyGameInstance)
            (:Is%20Valid
              (Development|PrintString (Utilities|GetDisplayName (Variables|Default|GetMyGameInstance))))
            (:Is%20Not%20Valid
              (Development|PrintString "RefMan: MyGameInstance is not valid B"))))))
    (:then_3
      ;[1 1 1] Game Mode (Parent and Individual ref)
      ;;[1 1 1] Clear all refs
      (Variables|Default|SetGame%20Mode%20Town 0)
      (Variables|Default|SetGame%20Mode%20Wild 0)
      ;;[1 1 1] Save ParentMode and current GM refs
      (bind _asgm_parent_mode (Utilities|Casting|CastToGM_ParentMode (Game|GetGameMode)))
      (bind _output_get (Variables|Default|SetGame%20Mode%20Parent _asgm_parent_mode))
      (bind _asgm_town (Utilities|Casting|CastToGM_Town _output_get)
        (:then
          (bind _output_get_2 (Variables|Default|SetGame%20Mode%20Town _asgm_town))
          (Development|PrintText (Utilities|Text|FormatText "Game Mode: {a}" (Utilities|Text|ToText(String) (Utilities|GetDisplayName _output_get_2)))))
        (:CastFailed
          (bind _asgm_wild (Utilities|Casting|CastToGM_Wild _output_get))
          (bind _output_get_3 (Variables|Default|SetGame%20Mode%20Wild _asgm_wild))
          (Development|PrintText (Utilities|Text|FormatText "Game Mode: {a}" (Utilities|Text|ToText(String) (Utilities|GetDisplayName _output_get_3)))))))
    (:then_5
      ;[1 1 1] Camera Manager
      (bind _outactors (Actor|GetAllActorswithTag "Camera Manager"))
      ;;[1 1 1] DEBUG
      (Utilities|IsValid (Utilities|Array|Get(acopy) _outactors)
        (:Is%20Valid
          (bind _ascamera_manager (Utilities|Casting|CastToCamera_Manager (Utilities|Array|Get(acopy) _outactors)))
          (Variables|Default|SetCamera%20Manager _ascamera_manager))))
    (:then_7
      ;[1 1 1] Popup Widget Manager
      (bind _outactors_2 (Actor|GetAllActorswithTag "Popup Widget Manager"))
      ;;[1 1 1] DEBUG
      (Utilities|IsValid (Utilities|Array|Get(acopy) _outactors_2)
        (:Is%20Valid
          (bind _aspopup_widget_manager (Utilities|Casting|CastToPopup_Widget_Manager (Utilities|Array|Get(acopy) _outactors_2)))
          (Variables|Default|SetPopup%20Widget%20Manager _aspopup_widget_manager))))
    (:then_9
      ;[1 1 1] HUD Manager
      (bind _outactors_3 (Actor|GetAllActorswithTag "HUD Manager"))
      ;;[1 1 1] DEBUG
      (Utilities|IsValid (Utilities|Array|Get(acopy) _outactors_3)
        (:Is%20Valid
          (bind _ashud_manager (Utilities|Casting|CastToHUD_Manager (Utilities|Array|Get(acopy) _outactors_3)))
          (Variables|Default|SetHUD%20Manager _ashud_manager))))
    (:then_11
      ;[1 1 1] PC Controller
      (bind _asmy_player_controller (Utilities|Casting|CastToMyPlayerController (Game|GetPlayerController 0)))
      (Variables|Default|SetMyPlayerController%20ref _asmy_player_controller))
    (:then_13
      ;[1 1 1] Player Character
      (bind _outactors_4 (Actor|GetAllActorswithTag "Player Character"))
      (Utilities|IsValid (Utilities|Array|Get(acopy) _outactors_4)
        (:Is%20Valid
          (bind _asyusa_3c_bp (Utilities|Casting|CastToyusa3C_BP (Utilities|Array|Get(acopy) _outactors_4)))
          (Variables|Default|SetYusa%20Character%20Reference _asyusa_3c_bp))
        (:Is%20Not%20Valid)))
    (:then_15
      ;[1 1 1] Dialogue Manager
      (bind _outactors_5 (Actor|GetAllActorswithTag "Dialogue Manager"))
      ;;[1 1 1] DEBUG
      (Utilities|IsValid (Utilities|Array|Get(acopy) _outactors_5)
        (:Is%20Valid
          (bind _asdialogue_manager (Utilities|Casting|CastToDialogue_Manager (Utilities|Array|Get(acopy) _outactors_5)))
          (Variables|Default|SetDialogue%20Manager _asdialogue_manager))))))
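; Manager that creates and drives dialogue popup widgets for NPC and portal conversations.
; DialoguePopupCreate resets the caller's completion flag, spawns a words-only or response widget, and positions it from X/Y presets, tracking popups per screen side.
; Companion functions fill the current popup's text and speaker arrays, then hand off to the widget's PrintDirector for display.
; Much of the EventGraph duplicates these functions, including a disconnected copy of the creation logic.
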(event Custom|CustomEvent_1
  (params (TextToDisplay :type String) (Speaker :type String) (DialogueForBranch :type Array%20of%20Strings))
  (bind _dialoguepopref_current (Variables|Default|GetdialoguePopRef_current))
  (bind _dialoguepopref_current_2 (Variables|Default|GetdialoguePopRef_current))
  ;[1 1 1] dialoguePopupAddScripts
  (Utilities|Array|Clear (Variables|/Game/0Project/Blueprints/Widgets/dialogue/dialoguePopupA2.dialoguePopupA2_C|GetText%20to%20Display _dialoguepopref_current_2))
  (Utilities|Array|Clear (Variables|/Game/0Project/Blueprints/Widgets/dialogue/dialoguePopupA2.dialoguePopupA2_C|GetText%20to%20Display%20Speaker _dialoguepopref_current_2))
  (for _array_element DialogueForBranch
    (Utilities|Array|Add (Variables|/Game/0Project/Blueprints/Widgets/dialogue/dialoguePopupA2.dialoguePopupA2_C|GetText%20to%20Display _dialoguepopref_current) _array_element)
    (Utilities|Array|Add (Variables|/Game/0Project/Blueprints/Widgets/dialogue/dialoguePopupA2.dialoguePopupA2_C|GetText%20to%20Display%20Speaker _dialoguepopref_current) Speaker)))

(event Custom|CustomEvent_3
  (params (TextToDisplay :type String) (Speaker :type String))
  (bind _dialoguepopref_current (Variables|Default|GetdialoguePopRef_current))
  ;[1 1 1] dialoguePopupAddResponse
  (Utilities|Array|Add (Variables|/Game/0Project/Blueprints/Widgets/dialogue/dialoguePopupA2.dialoguePopupA2_C|GetText%20to%20Display _dialoguepopref_current) TextToDisplay)
  (Utilities|Array|Add (Variables|/Game/0Project/Blueprints/Widgets/dialogue/dialoguePopupA2.dialoguePopupA2_C|GetText%20to%20Display%20Speaker _dialoguepopref_current) Speaker))

(event Custom|CustomEvent_4
  (params (Window%20Type :type EdialoguePopupWindowType%20Enum :default "NewEnumerator0") (CallerOfWidget :type Npc%20Parent%20Object%20Reference))
  ;[1 1 1] dialoguePopupClearAndPrintResponses
  ;[1 1 1] Print Director call
  (Default|PrintDirector (Variables|Default|GetdialoguePopRef_current) "NewEnumerator0" Window%20Type CallerOfWidget))

(event Custom|CustomEvent_2
  (params (Window%20Type :type EdialoguePopupWindowType%20Enum :default "NewEnumerator0") (CallerOfWidget :type Npc%20Parent%20Object%20Reference))
  ;[1 1 1] dialoguePopupClearAndPrintScript
  ;[1 1 1] Print Director call
  (Default|PrintDirector (Variables|Default|GetdialoguePopRef_current) "NewEnumerator0" Window%20Type CallerOfWidget (Variables|Default|GetCaller%20Of%20Widget%20%28Portal%29)))

(event EventBeginPlay
  ;[1 1 1] Event BeginPlay
  ;[0.4948 1 0.4405] Save Reference Manager ref
  ; - Place first so refs are available
  (bind _outactors (Actor|GetAllActorswithTag "Reference Manager"))
  (bind _asreference_manager (Utilities|Casting|CastToReference_Manager (Utilities|Array|Get(acopy) _outactors)))
  (Variables|Default|SetReference%20Manager _asreference_manager))

(fn ConstructionScript)

(fn DialoguePopup-Create
  (params (Dialogue%20Popup%20Settings :type S%20Dialogue%20Popup%20Settings%20Structure) (Caller%20of%20Widget%20%28NPC%29 :type Npc%20Parent%20Object%20Reference) (Caller%20of%20Widget%20%28Portal%29 :type BP%20Portal%20Parent%20Object%20Reference))
  ;[1 1 1] Save Dialogue Popup specs in struct
  (Variables|Default|SetDialogue%20Popup%20Settings "")
  ;[1 1 1] is Caller of Widget [NPC Parent Object] ref Valid?
  (Utilities|IsValid Caller%20of%20Widget%20%28NPC%29
    (:Is%20Valid
      (bind _output_get (Variables|Default|SetcallerOfWidget Caller%20of%20Widget%20%28NPC%29))
      (Variables|/Game/0Project/Blueprints/NPC/npcParent.npcParent_C|SetisDialogueComplete? _output_get false))
    (:Is%20Not%20Valid
      ;[1 1 1] is Caller of Widget(Portal) [BP Portal Parent Object] red Valid?
      (Utilities|IsValid Caller%20of%20Widget%20%28Portal%29
        (:Is%20Valid
          (bind _output_get_2 (Variables|Default|SetCaller%20Of%20Widget%20%28Portal%29 Caller%20of%20Widget%20%28Portal%29))
          (Variables|/Game/0Project/Blueprints/Interactables/Portals/BP_PortalParent.BP_PortalParent_C|SetisDialogueComplete? _output_get_2 false))
        (:Is%20Not%20Valid
          _))))
  (Variables|/Script/Engine.PlayerController|SetbShowMouseCursor (Game|GetPlayerController 0) false)
  ;[1 1 1] switch on dialogue Type [enum]
  (switch Utilities|FlowControl|Switch|SwitchonEdialoguePopupConvoType (.conversationtype (Variables|Default|GetDialogue%20Popup%20Settings))
    (:NewEnumerator0
      ;[1 1 1] Words Only method
      ;;[1 1 1] Switch on Window Type
      (switch Utilities|FlowControl|Switch|SwitchonEdialoguePopupWindowType (.windowtype (Variables|Default|GetDialogue%20Popup%20Settings))
        (:NewEnumerator0
          ;;[1 1 1] Create Normal 3-4 Lines Window Type
          (bind _returnvalue (UserInterface|CreateWidget "/Game/0Project/Blueprints/Widgets/dialogue/dialoguePopupA2.dialoguePopupA2_C"))
          (Variables|Default|SetdialoguePopRef_current _returnvalue)
          (Utilities|IsValid (Variables|Default|GetcallerOfWidget)
            (:Is%20Valid
              (bind _output_get_3 (Variables|/Game/0Project/Blueprints/Widgets/dialogue/dialoguePopup_Parent_BP.dialoguePopup_Parent_BP_C|SetCurrent%20String%20Speaker (Variables|Default|GetdialoguePopRef_current) (Variables|/Game/0Project/Blueprints/NPC/npcParent.npcParent_C|GetMyName_dialog (Variables|Default|GetcallerOfWidget))))
              (Rendering|Components|TextRender|SetText (Variables|/Game/0Project/Blueprints/Widgets/dialogue/dialoguePopupA2.dialoguePopupA2_C|GetNameHeader _returnvalue) (Utilities|Text|ToText(String) _output_get_3)))
            (:Is%20Not%20Valid
              (Rendering|Components|TextRender|SetText (Variables|/Game/0Project/Blueprints/Widgets/dialogue/dialoguePopupA2.dialoguePopupA2_C|GetNameHeader _returnvalue) ""))))
        (:NewEnumerator1
          ;;[1 1 1] Create Larger More Text Window Type
          (bind _returnvalue_2 (UserInterface|CreateWidget "/Game/0Project/Blueprints/Widgets/dialogue/dialoguePopupA1.dialoguePopupA1_C"))
          (Variables|Default|SetdialoguePopRef_current _returnvalue_2)
          (Utilities|IsValid (Variables|Default|GetcallerOfWidget)
            (:Is%20Valid
              (bind _output_get_4 (Variables|/Game/0Project/Blueprints/Widgets/dialogue/dialoguePopup_Parent_BP.dialoguePopup_Parent_BP_C|SetCurrent%20String%20Speaker (Variables|Default|GetdialoguePopRef_current) (Variables|/Game/0Project/Blueprints/NPC/npcParent.npcParent_C|GetMyName_dialog (Variables|Default|GetcallerOfWidget))))
              (Rendering|Components|TextRender|SetText (Variables|/Game/0Project/Blueprints/Widgets/dialogue/dialoguePopupA1.dialoguePopupA1_C|GetNameHeader _returnvalue_2) (Utilities|Text|ToText(String) _output_get_4)))
            (:Is%20Not%20Valid
              (Rendering|Components|TextRender|SetText (Variables|/Game/0Project/Blueprints/Widgets/dialogue/dialoguePopupA1.dialoguePopupA1_C|GetNameHeader _returnvalue_2) "")))))
      (UserInterface|Viewport|AddtoViewport (Variables|Default|GetdialoguePopRef_current) 0)
      (Widget|Transform|SetRenderScale (Variables|Default|GetdialoguePopRef_current) "(X=0.750000,Y=0.750000)")
      (Input|SetInputModeGameandUI (Game|GetPlayerController 0) 0 "DoNotLock" true)
      ;;[1 1 1] Set X position based on enums
      (Variables|Default|SetDialogue%20Popup%20XY%20Calc (Math|Vector2D|MakeVector2D (/ (Math|Conversions|ToFloat(Integer) (.SizeX (HUD|GetViewportSize (Game|GetPlayerController 0)))) 2.0) 0.0))
      (switch Utilities|FlowControl|Switch|SwitchonE_Popup_X_Position_Presets (.xpositionpreset (Variables|Default|GetDialogue%20Popup%20Settings))
        (:NewEnumerator0
          (Variables|Default|SetDialogue%20Popup%20Alignment "(X=0.950000,Y=-0.500000)")
          (Utilities|IsValid (Variables|Default|GetdialoguePopRef_LHS_1)
            (:Is%20Valid
              (if (== (Variables|Default|GetdialoguePopRef_current) (Variables|Default|GetdialoguePopRef_LHS_1))
                _
                (else
                  (Variables|Default|SetdialoguePopRef_LHS_2 (Variables|Default|GetdialoguePopRef_current)))))
            (:Is%20Not%20Valid
              (Variables|Default|SetdialoguePopRef_LHS_1 (Variables|Default|GetdialoguePopRef_current)))))
        (:NewEnumerator2
          (Variables|Default|SetDialogue%20Popup%20Alignment "(X=0.500000,Y=-0.500000)")
          (Utilities|IsValid (Variables|Default|GetdialoguePopRef_MID_1)
            (:Is%20Valid
              (if (== (Variables|Default|GetdialoguePopRef_current) (Variables|Default|GetdialoguePopRef_MID_1))
                _
                (else
                  (Variables|Default|SetdialoguePopRef_MID_2 (Variables|Default|GetdialoguePopRef_current)))))
            (:Is%20Not%20Valid
              (Variables|Default|SetdialoguePopRef_MID_1 (Variables|Default|GetdialoguePopRef_current)))))
        (:NewEnumerator1
          (Variables|Default|SetDialogue%20Popup%20Alignment "(X=0.050000,Y=-0.500000)")
          (Utilities|IsValid (Variables|Default|GetdialoguePopRef_RHS_1)
            (:Is%20Valid
              (if (== (Variables|Default|GetdialoguePopRef_current) (Variables|Default|GetdialoguePopRef_RHS_1))
                _
                (else
                  (Variables|Default|SetdialoguePopRef_RHS_2 (Variables|Default|GetdialoguePopRef_current)))))
            (:Is%20Not%20Valid
              (Variables|Default|SetdialoguePopRef_RHS_1 (Variables|Default|GetdialoguePopRef_current))))))
      (Variables|Default|SetdialoguePopRef_current (Variables|Default|GetdialoguePopRef_current))
      ;;[1 1 1] Set Y position based on enums
      (switch Utilities|FlowControl|Switch|SwitchonE_Popup_Y_Position_Presets (.ypositionpreset (Variables|Default|GetDialogue%20Popup%20Settings))
        (:NewEnumerator1
          (Variables|Default|SetDialogue%20Popup%20XY%20Calc (Math|Vector2D|MakeVector2D (.X (Math|Vector2D|BreakVector2D (Variables|Default|GetDialogue%20Popup%20XY%20Calc))) 3e+01)))
        (:NewEnumerator0
          (Variables|Default|SetDialogue%20Popup%20XY%20Calc (Math|Vector2D|MakeVector2D (.X (Math|Vector2D|BreakVector2D (Variables|Default|GetDialogue%20Popup%20XY%20Calc))) 1e+02))))
      ;;[1 1 1] Set Position and Alignment of Popup
      (Class|UserWidget|SetPositioninViewport (Variables|Default|GetdialoguePopRef_current) (Variables|Default|GetDialogue%20Popup%20XY%20Calc) true)
      (Class|UserWidget|SetAlignmentinViewport (Variables|Default|GetdialoguePopRef_current) (Variables|Default|GetDialogue%20Popup%20Alignment))
      ;;[1 1 1] Widget Appear
      (Default|AppearTypeRedirect (Variables|Default|GetdialoguePopRef_current) (.appearanimtype (Variables|Default|GetDialogue%20Popup%20Settings)) "NewEnumerator0" "NewEnumerator0"))
    (:NewEnumerator1
      ;[1 1 1] User Response method
      ;;[1 1 1] switch on Window Type
      (switch Utilities|FlowControl|Switch|SwitchonEdialoguePopupWindowType "NewEnumerator0"
        (:NewEnumerator0
          (bind _returnvalue_3 (UserInterface|CreateWidget "/Game/0Project/Blueprints/Widgets/dialogue/dialoguePopupA2_Response.dialoguePopupA2_Response_C"))
          (bind _output_get_5 (Variables|Default|SetdialoguePopRef_current _returnvalue_3))
          (bind _output_get_6 (Variables|/Game/0Project/Blueprints/Widgets/dialogue/dialoguePopup_Parent_BP.dialoguePopup_Parent_BP_C|SetCurrent%20String%20Speaker _output_get_5 (Variables|/Game/0Project/Blueprints/NPC/npcParent.npcParent_C|GetMyName_dialog (Variables|Default|GetcallerOfWidget))))
          (Rendering|Components|TextRender|SetText (Variables|/Game/0Project/Blueprints/Widgets/dialogue/dialoguePopupA2_Response.dialoguePopupA2_Response_C|GetNameHeader _returnvalue_3) (Utilities|Text|ToText(String) _output_get_6))
          (UserInterface|Viewport|AddtoViewport _output_get_5 0)
          (Widget|Transform|SetRenderScale _output_get_5 "(X=0.750000,Y=0.750000)")
          ;;[1 1 1] Set XY position based on enums
          (Variables|Default|SetDialogue%20Popup%20XY%20Calc (Math|Vector2D|MakeVector2D (/ (Math|Conversions|ToFloat(Integer) (.SizeX (HUD|GetViewportSize (Game|GetPlayerController 0)))) 2.0) 0.0))
          (switch Utilities|FlowControl|Switch|SwitchonE_Popup_X_Position_Presets (.xpositionpreset (Variables|Default|GetDialogue%20Popup%20Settings))
            (:NewEnumerator0
              (Variables|Default|SetDialogue%20Popup%20Alignment "(X=0.950000,Y=-0.500000)")
              (Utilities|IsValid (Variables|Default|GetdialoguePopRef_LHS_1)
                (:Is%20Valid
                  (if (== (Variables|Default|GetdialoguePopRef_current) (Variables|Default|GetdialoguePopRef_LHS_1))
                    _
                    (else
                      (Variables|Default|SetdialoguePopRef_LHS_2 (Variables|Default|GetdialoguePopRef_current)))))
                (:Is%20Not%20Valid
                  (Variables|Default|SetdialoguePopRef_LHS_1 (Variables|Default|GetdialoguePopRef_current)))))
            (:NewEnumerator2
              (Variables|Default|SetDialogue%20Popup%20Alignment "(X=0.500000,Y=-0.500000)")
              (Utilities|IsValid (Variables|Default|GetdialoguePopRef_MID_1)
                (:Is%20Valid
                  (if (== (Variables|Default|GetdialoguePopRef_current) (Variables|Default|GetdialoguePopRef_MID_1))
                    _
                    (else
                      (Variables|Default|SetdialoguePopRef_MID_2 (Variables|Default|GetdialoguePopRef_current)))))
                (:Is%20Not%20Valid
                  (Variables|Default|SetdialoguePopRef_MID_1 (Variables|Default|GetdialoguePopRef_current)))))
            (:NewEnumerator1
              (Variables|Default|SetDialogue%20Popup%20Alignment "(X=0.050000,Y=-0.500000)")
              (Utilities|IsValid (Variables|Default|GetdialoguePopRef_RHS_1)
                (:Is%20Valid
                  (if (== (Variables|Default|GetdialoguePopRef_current) (Variables|Default|GetdialoguePopRef_RHS_1))
                    _
                    (else
                      (Variables|Default|SetdialoguePopRef_RHS_2 (Variables|Default|GetdialoguePopRef_current)))))
                (:Is%20Not%20Valid
                  (Variables|Default|SetdialoguePopRef_RHS_1 (Variables|Default|GetdialoguePopRef_current))))))
          (Variables|Default|SetdialoguePopRef_current (Variables|Default|GetdialoguePopRef_current))
          (switch Utilities|FlowControl|Switch|SwitchonE_Popup_Y_Position_Presets (.ypositionpreset (Variables|Default|GetDialogue%20Popup%20Settings))
            (:NewEnumerator1
              (Variables|Default|SetDialogue%20Popup%20XY%20Calc (Math|Vector2D|MakeVector2D (.X (Math|Vector2D|BreakVector2D (Variables|Default|GetDialogue%20Popup%20XY%20Calc))) 3e+01)))
            (:NewEnumerator0
              (Variables|Default|SetDialogue%20Popup%20XY%20Calc (Math|Vector2D|MakeVector2D (.X (Math|Vector2D|BreakVector2D (Variables|Default|GetDialogue%20Popup%20XY%20Calc))) 1e+02))))
          (Class|UserWidget|SetPositioninViewport (Variables|Default|GetdialoguePopRef_current) (Variables|Default|GetDialogue%20Popup%20XY%20Calc) true)
          (Class|UserWidget|SetAlignmentinViewport (Variables|Default|GetdialoguePopRef_current) (Variables|Default|GetDialogue%20Popup%20Alignment)))
        (:NewEnumerator1)))))

(fn DialoguePopup-AddScripts
  (params (Text%20to%20Display :type String) (Speaker :type String) (Dialogue%20for%20Branch :type Array%20of%20Strings))
  (bind _dialoguepopref_current (Variables|Default|GetdialoguePopRef_current))
  (bind _dialoguepopref_current_2 (Variables|Default|GetdialoguePopRef_current))
  ;[1 1 1] dialoguePopupAddScripts
  (Utilities|Array|Clear (Variables|/Game/0Project/Blueprints/Widgets/dialogue/dialoguePopupA2.dialoguePopupA2_C|GetText%20to%20Display _dialoguepopref_current_2))
  (Utilities|Array|Clear (Variables|/Game/0Project/Blueprints/Widgets/dialogue/dialoguePopupA2.dialoguePopupA2_C|GetText%20to%20Display%20Speaker _dialoguepopref_current_2))
  (for _array_element Dialogue%20for%20Branch
    (Utilities|Array|Add (Variables|/Game/0Project/Blueprints/Widgets/dialogue/dialoguePopupA2.dialoguePopupA2_C|GetText%20to%20Display _dialoguepopref_current) _array_element)
    (Utilities|Array|Add (Variables|/Game/0Project/Blueprints/Widgets/dialogue/dialoguePopupA2.dialoguePopupA2_C|GetText%20to%20Display%20Speaker _dialoguepopref_current) Speaker)))

(fn DialoguePopup-ClearandPrintScripts
  (params (Window%20Type :type EdialoguePopupWindowType%20Enum :default "NewEnumerator0") (Caller%20of%20Widget%20%28NPC%29 :type Npc%20Parent%20Object%20Reference))
  ;[1 1 1] Print Director call
  (Default|PrintDirector (Variables|Default|GetdialoguePopRef_current) "NewEnumerator0" Window%20Type Caller%20of%20Widget%20%28NPC%29 (Variables|Default|GetCaller%20Of%20Widget%20%28Portal%29)))

(fn DialoguePopup-AddResponse
  (params (Text%20To%20Display :type String) (Speaker :type String))
  (bind _dialoguepopref_current (Variables|Default|GetdialoguePopRef_current))
  (Utilities|Array|Add (Variables|/Game/0Project/Blueprints/Widgets/dialogue/dialoguePopupA2.dialoguePopupA2_C|GetText%20to%20Display _dialoguepopref_current) Text%20To%20Display)
  (Utilities|Array|Add (Variables|/Game/0Project/Blueprints/Widgets/dialogue/dialoguePopupA2.dialoguePopupA2_C|GetText%20to%20Display%20Speaker _dialoguepopref_current) Speaker))

(fn DialoguePopup-ClearandPrintResponse
  (params (Window%20Type :type EdialoguePopupWindowType%20Enum :default "NewEnumerator0") (Caller%20of%20Widget%20%28NPC%29 :type Npc%20Parent%20Object%20Reference))
  ;[1 1 1] Print Director call
  (Default|PrintDirector (Variables|Default|GetdialoguePopRef_current) "NewEnumerator0" Window%20Type Caller%20of%20Widget%20%28NPC%29))
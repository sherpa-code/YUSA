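; Point light Blueprint that flickers by randomly varying its intensity during play.
; On BeginPlay it applies the configured light color and starts a fast looping timer that calls lightFlicker.
; Each tick of that timer rolls a random integer, and only some results set a new random intensity between IntensityMin and IntensityMax, so the flicker is irregular.
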(event Custom|lightFlicker
  (switch int (Math|Random|RandomIntegerinRange 0 4)
    (:0
      _)
    (:1
      _)
    (:2
      _))
  (Rendering|Components|Light|SetIntensity (Variables|Default|GetPointLight) (Math|Random|RandomFloatinRange (Variables|Default|Getintensity_min) (Variables|Default|Getintensity_max))))

(event EventBeginPlay
  (Rendering|Components|Light|SetLightColor (Variables|Default|GetPointLight) (Math|Conversions|ToLinearColor(Color) (Variables|Default|GetlightColor)) true)
  (Utilities|Time|SetTimerbyFunctionName 0 "lightFlicker" 0.05 true))

(fn ConstructionScript)
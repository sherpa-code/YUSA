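; RescueCrystal_A is a crystal actor that spins and flickers like a glowing jewel.
; BeginPlay starts a fast looping timer that calls fieldLightVariation, which randomly re-rolls the inner jewel's emissive strength and the point light's intensity, each only on some passes.
; Tick adds a fixed rotation every frame, unscaled by delta time.
; The dynamic material instance setup is disconnected; the emissive parameter is set directly on the mesh's materials.
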(event Custom|fieldLightVariation
  (Utilities|FlowControl|Sequence
    (:then_0
      (switch int (Math|Random|RandomIntegerinRange 0 4)
        (:0
          _)
        (:1
          _))
      (Rendering|Material|SetScalarParameterValueonMaterials (Variables|Default|GetJewelMeshInner) "Emissive Color Strength" (Math|Random|RandomFloatinRange 1e+01 9e+01)))
    (:then_1
      (switch int (Math|Random|RandomIntegerinRange 0 4)
        (:0
          _)
        (:1
          _))
      (Rendering|Material|SetScalarParameterValueonMaterials (Variables|Default|GetJewelMeshInner) "Emissive Color Strength" (Math|Random|RandomFloatinRange 17.0 75.0)))
    (:then_2
      (switch int (Math|Random|RandomIntegerinRange 0 4)
        (:0
          _)
        (:1
          _))
      (Rendering|Components|Light|SetIntensity (Variables|Default|GetPointLight) (Math|Random|RandomFloatinRange 3e+03 1.4e+04)))))

(event EventBeginPlay
  (Utilities|Time|SetTimerbyFunctionName 0 "fieldLightVariation" 0.05 true))

(event Collision|EventActorBeginOverlap
  (params (OtherActor :type Actor%20Object%20Reference)))

(event EventTick
  (params (DeltaSeconds :type Float%20%28single-precision%29))
  (Class|Actor|AddActorWorldRotation "0,1.000000, 0"))

(fn ConstructionScript)
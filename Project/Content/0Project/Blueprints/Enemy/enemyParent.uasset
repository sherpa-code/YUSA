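; Parent enemy Blueprint handling stun, damage, death and coin drops, with health and stun bar updates.
; damageCalcApply adds stun, then during player melee attacks lowers HP, shows number popups and triggers hit recovery, stun (at 75+) or death.
; Child reactions are hard-wired through casts to magmaEle_BP rather than overrides.
; Death halts movement and flickers the mesh with a FlipFlop/Delay loop; deathAnimEnd spawns coins by denomination and destroys the actor.
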(event Custom|damageCalcApply
  (params (weaponRef :type Actor%20Object%20Reference) (actorHit :type Actor%20Object%20Reference) (damageTaken :type Integer) (damageType :type String) (lastHitChained :type Integer) (stunAmount :type Integer))
  (bind _returnvalue (+ damageTaken 0))
  (bind _returnvalue_2 (+ damageTaken 0))
  (bind _enemyhpwidget (Variables|Default|GetEnemyHPWidget))
  (bind _returnvalue_3 (Transformation|GetWorldTransform _enemyhpwidget))
  (bind _returnvalue_4 (- _returnvalue 0))
  (bind _returnvalue_5 (- _returnvalue_2 0))
  (bind _location (Math|Transform|BreakTransform _returnvalue_3))
  (bind _returnvalue_6 (+ _location "0, 0,-75.000000"))
  (bind _returnvalue_7 (Math|Transform|MakeTransform _returnvalue_6))
  ;[1 1 1] damageCalcApply (to self)
  (Class|HitReceivedInterface|SetStun(Message) self stunAmount actorHit)
  (Variables|Default|SetActorHit actorHit)
  (switch int lastHitChained
    (:1
      _)
    (:2
      _))
  (Variables|Default|Setroaming false)
  (bind _asyusa_3c_bp (Utilities|Casting|CastToyusa3C_BP (Game|GetPlayerCharacter 0)))
  (if (Variables|/Game/0Project/Blueprints/Chars/PC_YUSA/yusa3C_BP.yusa3C_BP_C|GetMeleeAttackA_active _asyusa_3c_bp)
    (Variables|Default|SetHP_Current (Math|Integer|Clamp(Integer) (- (Variables|Default|GetHP_Current) _returnvalue_4) 0 (- (Variables|Default|GetHP_Current) _returnvalue_4)))
    (bind _returnvalue_8 (AddComponent|AddWidgetComponent true _returnvalue_7))
    (bind _asnumber_popup_3 (Utilities|Casting|CastTonumberPopup_3 (UserInterface|GetUserWidgetObject _returnvalue_8)))
    (Default|NumberPopup _asnumber_popup_3 _returnvalue_4 "NewEnumerator1")
    (Effects|SpawnEmitteratLocation "/Game/0Project/Assets/InfinityBladeEffects/Effects/FX_Mobile/combat/P_DoubleTap_Untyped_Damage.P_DoubleTap_Untyped_Damage" (Transformation|GetWorldLocation (Variables|Collision|GetCapsuleComponent)) :!label _label)
    (if (Actor|ActorHasTag actorHit "magmaEle")
      (bind _asmagma_ele_bp (Utilities|Casting|CastTomagmaEle_BP actorHit))
      (if (> (Variables|Default|GetHP_Current) 0)
        (if (not (Variables|Default|Getstunned))
          (if (>= (Variables|Default|GetStun_Current) 75)
            (Development|PrintString "Stunned begin")
            (Default|StunnedBeginEnemyChild _asmagma_ele_bp)
            (elif (not (Variables|Default|GethitRecovering))
              (Default|HitRecoveryEnemyChild _asmagma_ele_bp))))
        (else
          (bind _output_get (Variables|Default|SetenemyMesh (Variables|/Script/Engine.Character|GetMesh _asmagma_ele_bp)))
          (CallFunction|Death _output_get))))
    (elif (Variables|/Game/0Project/Blueprints/Chars/PC_YUSA/yusa3C_BP.yusa3C_BP_C|GetMeleeAttackB_active _asyusa_3c_bp)
      (Variables|Default|SetHP_Current (Math|Integer|Clamp(Integer) (- (Variables|Default|GetHP_Current) _returnvalue_5) 0 (- (Variables|Default|GetHP_Current) _returnvalue_5)))
      (bind _returnvalue_9 (AddComponent|AddWidgetComponent true _returnvalue_7))
      (bind _asnumber_popup_3_2 (Utilities|Casting|CastTonumberPopup_3 (UserInterface|GetUserWidgetObject _returnvalue_9)))
      (Default|NumberPopup _asnumber_popup_3_2 _returnvalue_5 "NewEnumerator1")
      (goto _label))))

(event Custom|Death
  (params (enemyMesh :type Skeletal%20Mesh%20Component%20Object%20Reference))
  (bind _dizzyeffectref (Variables|Default|GetdizzyEffectRef))
  ;[1 1 1] Death
  ;;[1 1 1] Death
  ;;[1 1 1] will not call once flag is set
  (if (not (Variables|Default|GetisDead))
    (Variables|Default|SetisDead true)
    (Pawn|Components|CharacterMovement|DisableMovement (Variables|Character|GetCharacterMovement))
    (Variables|Default|SetactingStateSwitchTo 14)
    (Utilities|IsValid _dizzyeffectref
      (:Is%20Valid
        (Actor|DestroyActor _dizzyeffectref))
      (:Is%20Not%20Valid
        _))
    (Variables|Default|Setaggroed false)
    (Variables|Default|Setstunned false)
    (Variables|Default|Setengaged false)
    (Variables|Default|SethitRecovering false)
    (Variables|Default|SethitListening false)
    (Utilities|Time|SetTimerbyFunctionName 0 "checkForHit" 0.0)
    (Utilities|Time|SetTimerbyFunctionName 0 "stunTickDown" 0.0)
    (Components|Movement|StopMovementImmediately (Variables|Character|GetCharacterMovement))
    (Variables|Default|SetcombatMoveToPCFailCount 0)
    (bind _returnvalue (Effects|SpawnEmitteratLocation "/Game/StarterContent/Particles/P_Smoke.P_Smoke" (Transformation|GetWorldLocation (Variables|Collision|GetCapsuleComponent))))
    ;;[1 1 1] Think this is always failing
    (Utilities|IsValid (Variables|Default|GetenemyMesh) :!label _label
      (:Is%20Valid
        (Utilities|FlowControl|FlipFlop :!label _label_2
          (:A
            (Rendering|SetVisibility (Variables|Default|GetenemyMesh) false false)
            (Utilities|FlowControl|Delay 0.025)
            (goto _label_2))
          (:B
            (Rendering|SetVisibility (Variables|Default|GetenemyMesh) true false)
            (Utilities|FlowControl|Delay 0.025)
            (goto _label)))))))

(event Custom|destroyPointLight
  (params (Owner :type Actor%20Object%20Reference) (toDestroy :type Point%20Light%20Component%20Object%20Reference) (delay :type Float%20%28single-precision%29))
  ;[1 1 1] destroyPointLight
  (Utilities|FlowControl|Delay delay)
  (Utilities|IsValid toDestroy
    (:Is%20Valid
      (Components|DestroyComponent toDestroy)
      (Development|PrintString "Destroy Point Light Succeed"))
    (:Is%20Not%20Valid)))

(event Custom|deathAnimEnd
  ;[1 1 1] Death
  ;;[1 1 1] deathAnimEnd
  (Components|DestroyComponent (stale Custom|Death _returnvalue))
  (CallFunction|DropCoins)
  (Actor|DestroyActor))

(event Custom|setCrosshairVisbility
  (params (Input :type Boolean))
  (bind _crosshair_wc (Variables|Default|Getcrosshair_wc))
  (bind _returnvalue (UserInterface|GetUserWidgetObject _crosshair_wc))
  ;[1 1 1] setCrosshairVisibility
  (if Input
    (Widget|SetVisibility _returnvalue "Visible")
    (else
      (Widget|SetVisibility _returnvalue "Hidden"))))

(event Custom|stunTickDown
  ;[1 1 1] stunTickDown
  (if (> (Variables|Default|GetStun_Current) 0)
    (bind _output_get (Variables|Default|SetStun_Current (- (Variables|Default|GetStun_Current) 1)))
    (if (not (>= _output_get 75))
      (if (Variables|Default|Getstunned)
        (bind _asmagma_ele_bp (Utilities|Casting|CastTomagmaEle_BP (Variables|Default|GetActorHit)))
        (Default|StunnedEnd _asmagma_ele_bp)))))

(event EventSetStun
  (params (stun_points :type Integer) (actorHit :type Actor%20Object%20Reference))
  ;[1 1 1] Event Set Stun (interface defn)
  (Variables|Default|SetStun_Current (Math|Integer|Clamp(Integer) (+ (- (+ stun_points 0) 0) (Variables|Default|GetStun_Current)) 0 100)))

(fn ConstructionScript)

(fn DropCoins
  (bind _capsulecomponent (Variables|Collision|GetCapsuleComponent))
  (bind _returnvalue (Transformation|GetWorldLocation _capsulecomponent))
  (if (>= (/ (Variables|Default|GetcoinsHolding) 500) 1)
    (for _index (range 1 (/ (Variables|Default|GetcoinsHolding) 500))
      (Game|SpawnActorfromClass "/Game/0Project/Blueprints/Items/coins/coin_500_bp2.coin_500_bp2_C" (Math|Transform|MakeTransform _returnvalue "0, 0, 0" "0.025000,0.025000,0.025000") "Undefined" 0 0))
    (Variables|Default|SetcoinsHolding (- (Variables|Default|GetcoinsHolding) (* 500 (/ (Variables|Default|GetcoinsHolding) 500)))))
  (if (> (/ (Variables|Default|GetcoinsHolding) 100) 0)
    (for _index_2 (range 1 (/ (Variables|Default|GetcoinsHolding) 100))
      (Game|SpawnActorfromClass "/Game/0Project/Blueprints/Items/coins/coin_100_bp2.coin_100_bp2_C" (Math|Transform|MakeTransform _returnvalue "0, 0, 0" "0.017500,0.017500,0.017500") "Undefined" 0 0))
    (Variables|Default|SetcoinsHolding (- (Variables|Default|GetcoinsHolding) (* 100 (/ (Variables|Default|GetcoinsHolding) 100)))))
  (if (> (/ (Variables|Default|GetcoinsHolding) 50) 0)
    (for _index_3 (range 1 (/ (Variables|Default|GetcoinsHolding) 50))
      (Game|SpawnActorfromClass "/Game/0Project/Blueprints/Items/coins/coin_50_BP2.coin_50_BP2_C" (Math|Transform|MakeTransform _returnvalue "0, 0, 0" "0.012500,0.012500,0.012500") "Undefined" 0 0))
    (Variables|Default|SetcoinsHolding (- (Variables|Default|GetcoinsHolding) (* 50 (/ (Variables|Default|GetcoinsHolding) 50)))))
  (if (> (/ (Variables|Default|GetcoinsHolding) 10) 0)
    (for _index_4 (range 1 (/ (Variables|Default|GetcoinsHolding) 10))
      (Game|SpawnActorfromClass "/Game/0Project/Blueprints/Items/coins/coin_10_BP.coin_10_BP_C" (Math|Transform|MakeTransform _returnvalue "0, 0, 0" "0.010000,0.010000,0.010000") "Undefined" 0 0))))

(fn StatsUpdate
  (bind _hp_max (Variables|Default|GetHP_Max))
  (bind _hp_current (Variables|Default|GetHP_Current))
  (bind _stun_current (Variables|Default|GetStun_Current))
  (bind _stun_max (Variables|Default|GetStun_Max))
  (bind _returnvalue (Math|Conversions|ToFloat(Integer) _hp_current))
  (bind _returnvalue_2 (Math|Conversions|ToFloat(Integer) _hp_max))
  (bind _returnvalue_3 (Math|Conversions|ToFloat(Integer) _stun_current))
  (bind _returnvalue_4 (Math|Conversions|ToFloat(Integer) _stun_max))
  (bind _returnvalue_5 (/ _returnvalue_3 _returnvalue_4))
  (bind _returnvalue_6 (/ _returnvalue _returnvalue_2))
  (bind _returnvalue_7 (Math|Float|Clamp(Float) _returnvalue_6))
  (bind _returnvalue_8 (Math|Float|Clamp(Float) _returnvalue_5))
  ;[1 1 1] Stats Update
  (bind _asenemy_hp_2 (Utilities|Casting|CastToEnemyHP_2 (UserInterface|GetUserWidgetObject (Variables|Default|GetEnemyHPWidget))))
  (Progress|SetPercent (Variables|/Game/0Project/Blueprints/Widgets/EnemyHP_2.EnemyHP_2_C|GetHealth_Bar _asenemy_hp_2) _returnvalue_7)
  (Variables|Default|SetHealth_Pct _returnvalue_7)
  (Progress|SetPercent (Variables|/Game/0Project/Blueprints/Widgets/EnemyHP_2.EnemyHP_2_C|GetStun_Bar _asenemy_hp_2) _returnvalue_8)
  (Variables|Default|SetStun_Pct _returnvalue_8))
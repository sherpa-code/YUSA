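; Player character Blueprint for Yusa, holding mostly disconnected leftover logic in the graphs shown.
; The construction script only casts the game instance to MyGameInstance, under a note about debugging equipped captured skills; its CapturedSkills read and array-set nodes are unwired.
; In the event graph, an unreachable fragment would switch the acting state when movement changes from walking to falling.
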(fn ConstructionScript
  ;[1 1 1] Debug Captured Skill Equipped
  (bind _asmy_game_instance (Utilities|Casting|CastToMyGameInstance (Game|GetGameInstance))))
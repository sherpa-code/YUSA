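; Decorative candle holder prop for an ArchVis pack, with customizable metal, plastic and candle wax surfaces.
; The construction script creates a dynamic material instance for each of the static mesh's three material slots.
; Blueprint variables drive color, metalness and roughness on metal and plastic, plus color, roughness and subsurface color and opacity on the wax.
; It has no runtime logic.
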(event EventBeginPlay)

(event Collision|EventActorBeginOverlap
  (params (OtherActor :type Actor%20Object%20Reference)))

(event EventTick
  (params (DeltaSeconds :type Float%20%28single-precision%29)))

(fn ConstructionScript
  (bind _returnvalue (Rendering|Material|CreateDynamicMaterialInstance (Variables|Default|GetStaticMesh) 0 "/Game/0Project/Assets/ArchVisPolishPack02/Materials/M_AVP2_Metal.M_AVP2_Metal" :!class /Script/Engine.PrimitiveComponent))
  (Rendering|Material|SetScalarParameterValue _returnvalue "Metal.Metalness" (Variables|Metal|GetMetal.Metalness) :!class /Script/Engine.MaterialInstanceDynamic)
  (Rendering|Material|SetScalarParameterValue _returnvalue "Metal.Roughness" (Variables|Metal|GetMetal.Roughness) :!class /Script/Engine.MaterialInstanceDynamic)
  (Rendering|Material|SetVectorParameterValue _returnvalue "Metal.Color" (Variables|Metal|GetMetal.Color) :!class /Script/Engine.MaterialInstanceDynamic)
  (bind _returnvalue_2 (Rendering|Material|CreateDynamicMaterialInstance (Variables|Default|GetStaticMesh) 1 "/Game/0Project/Assets/ArchVisPolishPack02/Materials/M_AVP2_Plastic.M_AVP2_Plastic" :!class /Script/Engine.PrimitiveComponent))
  (Rendering|Material|SetScalarParameterValue _returnvalue_2 "Plastic.Metalness" (Variables|Plastic|GetPlastic.Metalness) :!class /Script/Engine.MaterialInstanceDynamic)
  (Rendering|Material|SetScalarParameterValue _returnvalue_2 "Plastic.Roughness" (Variables|Plastic|GetPlastic.Roughness) :!class /Script/Engine.MaterialInstanceDynamic)
  (Rendering|Material|SetVectorParameterValue _returnvalue_2 "Plastic.COlor" (Variables|Plastic|GetPlastic.Color) :!class /Script/Engine.MaterialInstanceDynamic)
  (bind _returnvalue_3 (Rendering|Material|CreateDynamicMaterialInstance (Variables|Default|GetStaticMesh) 2 "/Game/0Project/Assets/ArchVisPolishPack02/Materials/M_AVP2_CandleWax.M_AVP2_CandleWax" :!class /Script/Engine.PrimitiveComponent))
  (Rendering|Material|SetVectorParameterValue _returnvalue_3 "Wax.Color" (Variables|Wax|GetWax.Color) :!class /Script/Engine.MaterialInstanceDynamic)
  (Rendering|Material|SetVectorParameterValue _returnvalue_3 "Wax.SS_Color" (Variables|Wax|GetWax.SS_Color) :!class /Script/Engine.MaterialInstanceDynamic)
  (Rendering|Material|SetScalarParameterValue _returnvalue_3 "Wax.Roughness" (Variables|Wax|GetWax.Roughness) :!class /Script/Engine.MaterialInstanceDynamic)
  (Rendering|Material|SetScalarParameterValue _returnvalue_3 "Wax.SS_Opacity" (Variables|Wax|GetWax.SS_Opacity) :!class /Script/Engine.MaterialInstanceDynamic))
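; BP_AVP2_Candle_03 is a configurable candle prop with a static mesh, flickering flame particle and point light.
; Its construction script applies shadow casting, light radius and temperature, and uses Lit to toggle flame visibility and light intensity.
; It also creates a dynamic wax material instance to set color, roughness and subsurface color and opacity.
; The event graph holds only empty placeholder events, so there is no runtime logic.
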(event EventBeginPlay)

(event Collision|EventActorBeginOverlap
  (params (OtherActor :type Actor%20Object%20Reference)))

(event EventTick
  (params (DeltaSeconds :type Float%20%28single-precision%29)))

(fn ConstructionScript
  (bind _lit (Variables|CandleFlame|GetLit))
  (bind _pointlight (Variables|Default|GetPointLight))
  ;[1 1 1] Shadows
  (Rendering|SetCastShadow (Variables|Debug|GetStaticMeshComponent) (Variables|Default|GetCast%20Shadow))
  ;[1 1 1] Flame Particle
  (Rendering|SetVisibility (Variables|Default|GetP_FlameFlicker) _lit false)
  ;[1 1 1] Candle Light
  (if _lit
    (Rendering|Components|Light|SetIntensity _pointlight (Variables|CandleFlame|GetIntensity))
    (else
      (Rendering|Components|Light|SetIntensity _pointlight 0.0)))
  (Rendering|Lighting|SetAttenuationRadius _pointlight (Variables|CandleFlame|GetAttenuation%20Radius))
  (Class|LightComponent|SetTemperature _pointlight (Variables|CandleFlame|GetTemperature))
  ;[1 1 1] Candle Wax
  (bind _returnvalue (Rendering|Material|CreateDynamicMaterialInstance (Variables|Debug|GetStaticMeshComponent) 0 "/Game/0Project/Assets/ArchVisPolishPack02/Materials/M_AVP2_CandleWax.M_AVP2_CandleWax" :!class /Script/Engine.PrimitiveComponent))
  (Rendering|Material|SetVectorParameterValue _returnvalue "Wax.Color" (Variables|CandleWax|GetWax.Color) :!class /Script/Engine.MaterialInstanceDynamic)
  (Rendering|Material|SetVectorParameterValue _returnvalue "Wax.SS_Color" (Variables|CandleWax|GetWax.SS_Color) :!class /Script/Engine.MaterialInstanceDynamic)
  (Rendering|Material|SetScalarParameterValue _returnvalue "Wax.Roughness" (Variables|CandleWax|GetWax.Roughness) :!class /Script/Engine.MaterialInstanceDynamic)
  (Rendering|Material|SetScalarParameterValue _returnvalue "Wax.SS_Opacity" (Variables|CandleWax|GetWax.SS_Opacity) :!class /Script/Engine.MaterialInstanceDynamic))
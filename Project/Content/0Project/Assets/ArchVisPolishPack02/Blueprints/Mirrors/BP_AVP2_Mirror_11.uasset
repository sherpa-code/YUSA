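; BP_AVP2_Mirror_11 is a placeable mirror prop from the ArchVisPolishPack02 asset pack with adjustable mirror and plastic materials.
; Its construction script creates dynamic material instances from the mirror and plastic master materials on the mesh's first two slots.
; Blueprint variables drive metalness, roughness and color for each surface, so edits apply at construction time.
; The event graph holds only disabled stub events, so it has no runtime logic.
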(event EventBeginPlay)

(event Collision|EventActorBeginOverlap
  (params (OtherActor :type Actor%20Object%20Reference)))

(event EventTick
  (params (DeltaSeconds :type Float%20%28single-precision%29)))

(fn ConstructionScript
  (bind _returnvalue (Rendering|Material|CreateDynamicMaterialInstance (Variables|Default|GetStaticMesh) 0 "/Game/0Project/Assets/ArchVisPolishPack02/Materials/M_AVP2_Mirror.M_AVP2_Mirror" :!class /Script/Engine.PrimitiveComponent))
  (Rendering|Material|SetScalarParameterValue _returnvalue "Mirror.Metalness" (Variables|Mirror|GetMirror.Metalness) :!class /Script/Engine.MaterialInstanceDynamic)
  (Rendering|Material|SetScalarParameterValue _returnvalue "Mirror.Roughness" (Variables|Mirror|GetMirror.Roughness) :!class /Script/Engine.MaterialInstanceDynamic)
  (Rendering|Material|SetVectorParameterValue _returnvalue "Mirror.Color" (Variables|Mirror|GetMirror.Color) :!class /Script/Engine.MaterialInstanceDynamic)
  (bind _returnvalue_2 (Rendering|Material|CreateDynamicMaterialInstance (Variables|Default|GetStaticMesh) 1 "/Game/0Project/Assets/ArchVisPolishPack02/Materials/M_AVP2_Plastic.M_AVP2_Plastic" :!class /Script/Engine.PrimitiveComponent))
  (Rendering|Material|SetScalarParameterValue _returnvalue_2 "Plastic.Metalness" (Variables|Frame|GetPlastic.Metalness) :!class /Script/Engine.MaterialInstanceDynamic)
  (Rendering|Material|SetScalarParameterValue _returnvalue_2 "Plastic.Roughness" (Variables|Frame|GetPlastic.Roughness) :!class /Script/Engine.MaterialInstanceDynamic)
  (Rendering|Material|SetVectorParameterValue _returnvalue_2 "Plastic.Color" (Variables|Frame|GetPlastic.Color) :!class /Script/Engine.MaterialInstanceDynamic))
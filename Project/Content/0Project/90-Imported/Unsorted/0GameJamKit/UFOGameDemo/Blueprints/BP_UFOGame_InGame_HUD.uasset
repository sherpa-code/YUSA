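; In-game HUD for the UFO game demo, adding the UFO HUD widget on top of the menus its parent loads.
; BeginPlay calls the parent, then creates the in-game widget and adds it to the viewport.
; RegisterWin and RegisterLoss set the game over widget to its win or loss state, show it, and switch to UI-only input with the mouse cursor visible.
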(event EventBeginPlay
  (|CallParentFunction) ; Calling the Parent loads all the other HUD menus
  (Utilities|FlowControl|Sequence
    (:then_0
      ;[1 1 1] Add UFO HUD
      (bind _returnvalue (UserInterface|CreateWidget 0 (Game|Player|GetOwningPlayerController))) ; Then, you can add additional menus and widgets
      (bind _output_get (Variables|Default|SetMyInGameHUDWidget _returnvalue))
      (UserInterface|Viewport|AddtoViewport _output_get 0))))

(event EventRegisterLoss
  (bind _returnvalue (Game|GetPlayerController 0))
  (bind _mygameoverwidget (Variables|Default|GetMyGameOverWidget))
  (bind _mygameoverwidget_2 (Variables|Default|GetMyGameOverWidget)
    (:then
      (CallFunction|SetLoss _mygameoverwidget_2)
      (Widget|SetVisibility _mygameoverwidget "Visible")
      (Input|SetInputModeUIOnly _returnvalue _mygameoverwidget "DoNotLock")
      (Variables|/Script/Engine.PlayerController|SetbShowMouseCursor _returnvalue true))
    (:else)))

(event EventRegisterWin
  (bind _returnvalue (Game|GetPlayerController 0))
  (bind _mygameoverwidget (Variables|Default|GetMyGameOverWidget))
  (bind _mygameoverwidget_2 (Variables|Default|GetMyGameOverWidget)
    (:then
      (CallFunction|SetWin _mygameoverwidget_2)
      (Widget|SetVisibility _mygameoverwidget "Visible")
      (Input|SetInputModeUIOnly _returnvalue _mygameoverwidget "DoNotLock")
      (Variables|/Script/Engine.PlayerController|SetbShowMouseCursor _returnvalue true))
    (:else)))

(fn ConstructionScript
  (|CallParentFunction))
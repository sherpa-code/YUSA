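; Generic target actor from a game jam kit that awards the instigating controller a point when damaged.
; Construction creates a dynamic material instance on the static mesh and applies the configurable base color.
; The first damage event, gated by a DoOnce, recolors the material to glowing orange, turns off custom depth rendering and sends a score message to the instigator.
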(event EventBeginPlay)

(event Collision|EventActorBeginOverlap
  (params (OtherActor :type Actor%20Object%20Reference)))

(event EventTick
  (params (DeltaSeconds :type Float%20%28single-precision%29)))

(event Game|Damage|EventAnyDamage
  (params (Damage :type Float%20%28single-precision%29) (DamageType :type Damage%20Type%20Object%20Reference) (InstigatedBy :type Controller%20Object%20Reference) (DamageCauser :type Actor%20Object%20Reference))
  (bind _mymaterialinstance (Variables|Default|GetMyMaterialInstance))
  (|DoOnceMultiInput
    (:A%20Out
      (Rendering|Material|SetVectorParameterValue _mymaterialinstance "ColorBase" "(R=1.000000,G=0.556106,B=0.000000,A=1.000000)" :!class /Script/Engine.MaterialInstanceDynamic)
      (Rendering|Material|SetVectorParameterValue _mymaterialinstance "EmissiveCOlor" "(R=4.000000,G=0.032369,B=0.000000,A=1.000000)" :!class /Script/Engine.MaterialInstanceDynamic)
      (Rendering|SetRenderCustomDepth (Variables|Default|GetStaticMesh) false)
      (Class|Object|RegisterPlayerScore(Message) InstigatedBy 1.0) ; Tell the PC we scored!
    )))

(fn ConstructionScript
  (bind _returnvalue (Rendering|Material|CreateDynamicMaterialInstance (Variables|Default|GetStaticMesh) 0 0 "None" :!class /Script/Engine.PrimitiveComponent))
  (bind _output_get (Variables|Default|SetMyMaterialInstance _returnvalue))
  (Rendering|Material|SetVectorParameterValue _output_get "ColorBase" (Variables|Default|GetBaseColor) :!class /Script/Engine.MaterialInstanceDynamic))